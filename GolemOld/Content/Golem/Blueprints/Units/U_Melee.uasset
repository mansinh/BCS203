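; Melee golem unit that punches with randomly picked arm timelines and sphere-traces to damage and knock back Enemy-tagged actors.
; MeleeMerge keeps the best multipliers from the merged units, destroys the others and shows eligible skills on the melee widget.
; MeleeUpgrade applies the chosen skill from two chains: extra arms for offence or shields leading to Turtle Formation.
; BeginPlay currently grants the whole arm chain, up to Seraphim.
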(event Custom|RAttack
  (bind _right (Variables|Default|GetRight))
  (bind _left (Variables|Default|GetLeft))
  (bind _right1 (Variables|Default|GetRight1))
  (bind _left1 (Variables|Default|GetLeft1))
  (bind _right_2 (Variables|Default|GetRight))
  (bind _left_2 (Variables|Default|GetLeft))
  (bind _right1_2 (Variables|Default|GetRight1))
  (bind _left1_2 (Variables|Default|GetLeft1))
  ;[1 1 1] Attack animation?
  (switch int (Variables|Default|GetAttackingArm)
    (:0
      (Variables|Default|SetRAttacking true)
      (Transformation|SetWorldLocation (Variables|Default|GetRight) (Transformation|GetActorLocation (Variables|Default|GetTargetActor)) false false)
      (|CollapseGraph_0_2 _right)
      (Utilities|FlowControl|Delay 0.6)
      (|CollapseGraph_1_2 _right (Variables|Default|GetBody))
      (Transformation|SetRelativeLocation _right_2 "-22.000000,-10.000000,0.000000" false false)
      (Transformation|SetRelativeRotation _right_2 "40.000000,-15.000000,-70.000000" false false)
      (Variables|Default|SetRAttacking false))
    (:1
      (Variables|Default|SetR1Attacking true)
      (Transformation|SetWorldLocation (Variables|Default|GetRight1) (Transformation|GetActorLocation (Variables|Default|GetTargetActor)) false false)
      (|CollapseGraph_0_2_2_2 _right1)
      (Utilities|FlowControl|Delay 0.6)
      (|CollapseGraph_1_2_2_2 _right1 (Variables|Default|GetBody))
      (Transformation|SetRelativeLocation _right1_2 "-12.000000,-15.000000,40.000000" false false)
      (Transformation|SetRelativeRotation _right1_2 "20.000000, 0,-45.000000" false false)
      (Variables|Default|SetR1Attacking false))
    (:2
      (Variables|Default|SetL1Attacking true)
      (Transformation|SetWorldLocation (Variables|Default|GetLeft1) (Transformation|GetActorLocation (Variables|Default|GetTargetActor)) false false)
      (|CollapseGraph_0_2_2_2_2 _left1)
      (Utilities|FlowControl|Delay 0.6)
      (|CollapseGraph_1_2_2_2_2 _left1 (Variables|Default|GetBody))
      (Transformation|SetRelativeLocation _left1_2 "10.000000,-15.000000,40.000000" false false)
      (Transformation|SetRelativeRotation _left1_2 "-20.000000, 0,-45.000000" false false)
      (Variables|Default|SetL1Attacking false))
    (:3
      (Variables|Default|SetLAttacking true)
      (Transformation|SetWorldLocation (Variables|Default|GetLeft) (Transformation|GetActorLocation (Variables|Default|GetTargetActor)) false false)
      (|CollapseGraph_0_2_2 _left)
      (Utilities|FlowControl|Delay 0.6)
      (|CollapseGraph_1_2_2 _left (Variables|Default|GetBody))
      (Transformation|SetRelativeLocation _left_2 "20.000000,-10.000000,0.000000" false false)
      (Transformation|SetRelativeRotation _left_2 "40.000000,15.000000,-70.000000" false false)
      (Variables|Default|SetLAttacking false))))

(event Custom|Melee%20Merge
  (bind _asplayer_unit (Utilities|Casting|CastToPlayerUnit (Game|Player|GetPlayerPawn 0)))
  (Variables|Default|SetAs%20Player%20Unit _asplayer_unit)
  (Variables|Default|SetButtonholder (Variables|/Game/Golem/UI/MergeMenues/MeleeMergeMenu.MeleeMergeMenu_C|GetButtonholder (Variables|/Game/Golem/Blueprints/Units/PlayerUnit.PlayerUnit_C|GetMeleeWidget _asplayer_unit)))
  (if (== self (Variables|/Game/Golem/Blueprints/Units/PlayerUnit.PlayerUnit_C|GetMainMergeUnit (Variables|Default|GetAs%20Player%20Unit)))
    ;[1 1 1] Stat setting
    (for _array_element (Variables|/Game/Golem/Blueprints/Units/PlayerUnit.PlayerUnit_C|GetMergeUnits (Variables|Default|GetAs%20Player%20Unit))
      (if (> (Variables|/Game/Golem/Blueprints/Units/Unit.Unit_C|GetAttackDamageMultiplier _array_element) (Variables|Default|GetAttackDamageMultiplier))
        (Variables|Default|SetAttackDamageMultiplier (Variables|/Game/Golem/Blueprints/Units/Unit.Unit_C|GetAttackDamageMultiplier _array_element))))
    (for _array_element_2 (Variables|/Game/Golem/Blueprints/Units/PlayerUnit.PlayerUnit_C|GetMergeUnits (Variables|Default|GetAs%20Player%20Unit))
      (if (not (> (Variables|/Game/Golem/Blueprints/Units/Unit.Unit_C|GetAttackCoolDownMultiplier _array_element_2) (Variables|Default|GetAttackCoolDownMultiplier)))
        (Variables|Default|SetAttackCoolDownMultiplier (Variables|/Game/Golem/Blueprints/Units/Unit.Unit_C|GetAttackCoolDownMultiplier _array_element_2))))
    (for _array_element_3 (Variables|/Game/Golem/Blueprints/Units/PlayerUnit.PlayerUnit_C|GetMergeUnits (Variables|Default|GetAs%20Player%20Unit))
      (if (> (Variables|/Game/Golem/Blueprints/Units/Unit.Unit_C|GetDefenceMultiplier _array_element_3) (Variables|Default|GetDefenceMultiplier))
        (Variables|Default|SetDefenceMultiplier (Variables|/Game/Golem/Blueprints/Units/Unit.Unit_C|GetDefenceMultiplier _array_element_3))))
    (for _array_element_4 (Variables|/Game/Golem/Blueprints/Units/PlayerUnit.PlayerUnit_C|GetMergeUnits (Variables|Default|GetAs%20Player%20Unit))
      (if (> (Variables|/Game/Golem/Blueprints/Units/Unit.Unit_C|GetMaxHealthMultiplier _array_element_4) (Variables|Default|GetMaxHealthMultiplier))
        (Variables|Default|SetMaxHealthMultiplier (Variables|/Game/Golem/Blueprints/Units/Unit.Unit_C|GetMaxHealthMultiplier _array_element_4))))
    (bind _array_element_5 (Utilities|Array|ForEachLoopwithBreak (Variables|/Game/Golem/Blueprints/Units/PlayerUnit.PlayerUnit_C|GetMergeUnits (Variables|Default|GetAs%20Player%20Unit)))
      (:LoopBody
        (if (not (== _array_element_5 (Variables|/Game/Golem/Blueprints/Units/PlayerUnit.PlayerUnit_C|GetMainMergeUnit (Variables|Default|GetAs%20Player%20Unit))))
          (Actor|DestroyActor _array_element_5)))
      (:Completed
        ;[1 1 1] Adding skills (ints) to array
        (Utilities|Array|Clear (Variables|Default|GetAwailable%20skills))
        (for _index (range 0 5)
          (switch int _index
            (:0
              ;[1 1 1] Two Handed
              (if (not (Variables|Default|GetIsTwoHanded))
                (Utilities|Array|Add (Variables|Default|GetAwailable%20skills) (+ 0 0))))
            (:1
              ;[1 1 1] Shielded
              (if (not (Variables|Default|GetIsShielded))
                (Utilities|Array|Add (Variables|Default|GetAwailable%20skills) (+ 0 1))))
            (:2
              ;[1 1 1] Need Another arm?
              (if (Variables|Default|GetIsTwoHanded)
                (if (not (Variables|Default|GetIsNeedAnotherArm))
                  (Utilities|Array|Add (Variables|Default|GetAwailable%20skills) (+ 0 2)))))
            (:3
              ;[1 1 1] Reflected
              (if (Variables|Default|GetIsShielded)
                (if (not (Variables|Default|GetIsReflected))
                  (Utilities|Array|Add (Variables|Default|GetAwailable%20skills) (+ 0 3)))))
            (:4
              ;[1 1 1] Seraphim
              (if (Variables|Default|GetIsNeedAnotherArm)
                (if (not (Variables|Default|GetIsSeraphim))
                  (Utilities|Array|Add (Variables|Default|GetAwailable%20skills) (+ 0 4)))))
            (:5
              ;[1 1 1] Turtle Formation
              (if (Variables|Default|GetIsReflected)
                (if (not (Variables|Default|GetIsTurtle))
                  (Utilities|Array|Add (Variables|Default|GetAwailable%20skills) (+ 0 5)))))))
        ;[1 1 1] Creating buttons
        (for (_array_element_6 _array_index) (Variables|Default|GetAwailable%20skills)
          (for (_array_element_7 _array_index_2) (Class|PanelWidget|GetAllChildren (Variables|Default|GetButtonholder))
            (if (or (== (* _array_index 2) _array_index_2) (== (+ (* _array_index 2) 1) _array_index_2))
              (bind _astext (Utilities|Casting|CastToTextBlock _array_element_7)
                (:then
                  (Widget|SetVisibility _array_element_7 "Visible")
                  ;[1 1 1] Setting Text description
                  (switch int _array_element_6
                    (:0
                      (Rendering|Components|TextRender|SetText _astext "Two Handed"))
                    (:1
                      (Rendering|Components|TextRender|SetText _astext "Shielded"))
                    (:2
                      (Rendering|Components|TextRender|SetText _astext "Need Another Arm?"))
                    (:3
                      (Rendering|Components|TextRender|SetText _astext "Reflected"))
                    (:4
                      (Rendering|Components|TextRender|SetText _astext "Seraphim"))
                    (:5
                      (Rendering|Components|TextRender|SetText _astext "Turtle Formation"))))
                (:CastFailed
                  (Widget|SetVisibility _array_element_7 "Visible"))))))))))

(event Custom|MeleeUpgrade
  (bind _as_player_unit (Variables|Default|GetAs%20Player%20Unit))
  (bind _mainmergeunit (Variables|/Game/Golem/Blueprints/Units/PlayerUnit.PlayerUnit_C|GetMainMergeUnit _as_player_unit))
  ;[1 1 1] Checking Array and setting Corresponding Boolean (skill) to true
  (bind (_array_element _array_index) (Utilities|Array|ForEachLoopwithBreak (Variables|Default|GetAwailable%20skills) :!label _label)
    (:LoopBody
      (if (== _array_index (Variables|Default|GetASpos))
        (switch int _array_element
          (:0
            (CallFunction|TwoHanded))
          (:1
            (CallFunction|Shielded))
          (:2
            (CallFunction|NeedAnotherArm?))
          (:3
            (CallFunction|Reflected))
          (:4
            (CallFunction|Seraphim))
          (:5
            (CallFunction|Turtle)))
        (Variables|Default|SetASpos 0)
        (Variables|/Game/Golem/Blueprints/Units/Unit.Unit_C|SetMerges _mainmergeunit (+ (Variables|/Game/Golem/Blueprints/Units/Unit.Unit_C|GetMerges _mainmergeunit) 1))
        (Utilities|Array|Clear (Variables|/Game/Golem/Blueprints/Units/PlayerUnit.PlayerUnit_C|GetMergeUnits _as_player_unit))
        (for _array_element_2 (Class|PanelWidget|GetAllChildren (Variables|Default|GetButtonholder))
          (Widget|SetVisibility _array_element_2 "Collapsed"))
        (Widget|RemovefromParent (Variables|/Game/Golem/Blueprints/Units/PlayerUnit.PlayerUnit_C|GetMeleeWidget _as_player_unit))
        (Default|StopMerge (Variables|/Game/Golem/Blueprints/Units/PlayerUnit.PlayerUnit_C|GetUnitInformation _as_player_unit))
        (goto _label Break)))))

(event EventBeginPlay
  (CallFunction|Init)
  (CallFunction|TwoHanded)
  (CallFunction|NeedAnotherArm?)
  (CallFunction|Seraphim))

(event EventAttack
  (if (> (Variables|Default|GetHealth) 0.0)
    (if (> (Variables|Default|GetTimeSinceLastAttack) (* (Variables|Default|GetAttackCoolDown) (Variables|Default|GetAttackCoolDownMultiplier)))
      (Variables|Default|SetTimeSinceLastAttack 0.0)
      (CallFunction|AttackAnimation)
      (CallFunction|AttackAnimation)
      (if (== (Variables|Default|GetAttackArmCount) (Variables|Default|GetAttackingArm))
        (Variables|Default|SetAttackingArm 0)
        (else
          (Math|Integer|IncrementInt (Variables|Default|GetAttackingArm)
            (:%20%20
              (Utilities|FlowControl|Delay 0.16)
              (CallFunction|MeleeTarget))))))))

(fn ConstructionScript
  (bind _right_arm_anim (Variables|Default|GetRight%20Arm%20Anim))
  (bind _left_arm_anim (Variables|Default|GetLeft%20Arm%20Anim))
  (bind _right_arm_anim1 (Variables|Default|GetRight%20Arm%20Anim1))
  (bind _left_arm_anim1 (Variables|Default|GetLeft%20Arm%20Anim1))
  (|CallParentFunction)
  (Rendering|Material|SetMaterial (Variables|Default|GetcrystalMesh1) 0 (Variables|Default|GetCrystalMaterial))
  (Class|TimelineComponent|SetFloatCurve _right_arm_anim "/Game/Golem/Blueprints/PunchRotation.PunchRotation" "rotation")
  (Class|TimelineComponent|SetFloatCurve _right_arm_anim "/Game/Golem/Blueprints/PunchLocation.PunchLocation" "location")
  (Class|TimelineComponent|SetFloatCurve _left_arm_anim "/Game/Golem/Blueprints/PunchRotation.PunchRotation" "rotation")
  (Class|TimelineComponent|SetFloatCurve _left_arm_anim "/Game/Golem/Blueprints/PunchLocation.PunchLocation" "location")
  (Class|TimelineComponent|SetFloatCurve _right_arm_anim1 "/Game/Golem/Blueprints/PunchRotation.PunchRotation" "rotation")
  (Class|TimelineComponent|SetFloatCurve _right_arm_anim1 "/Game/Golem/Blueprints/PunchLocation.PunchLocation" "location")
  (Class|TimelineComponent|SetFloatCurve _left_arm_anim1 "/Game/Golem/Blueprints/PunchRotation.PunchRotation" "rotation")
  (Class|TimelineComponent|SetFloatCurve _left_arm_anim1 "/Game/Golem/Blueprints/PunchLocation.PunchLocation" "location"))

(fn MeleeTarget
  (bind _meleeattackimpact (Variables|Default|GetMeleeAttackImpact))
  (bind _outhits (Collision|MultiSphereTraceByChannel (Transformation|GetActorLocation) (Transformation|GetWorldLocation (Variables|Default|GetMeleeAttackPosition)) (Variables|Default|GetAttackRadius) "TraceTypeQuery2" false 0 "None"))
  (bind _array_element (Utilities|Array|ForEachLoopwithBreak _outhits)
    (:LoopBody
      (if (and (Utilities|DoesObjectImplementInterface (.HitActor (Collision|BreakHitResult _array_element)) "/Game/Golem/Blueprints/GolemInterface.GolemInterface_C") (Actor|ActorHasTag (.HitActor (Collision|BreakHitResult _array_element)) "Enemy"))
        (Transformation|SetWorldLocation _meleeattackimpact (.ImpactPoint (Collision|BreakHitResult _array_element)) false false)
        (Components|Activation|Activate _meleeattackimpact true)
        (bind _knockbackvector (CallFunction|GetKnockback (.HitActor (Collision|BreakHitResult _array_element))))
        (Class|GolemInterface|Attacked(Message) (.HitActor (Collision|BreakHitResult _array_element)) (* (Variables|Default|GetAttackDamage) (Variables|Default|GetAttackDamageMultiplier)) _knockbackvector)))))

(fn BlockAttack
  (bind _isblocked (|CallParentFunction))
  (return _isblocked))

(fn AttackAnimation
  (bind _attackarmcount (Variables|Default|GetAttackArmCount))
  (bind _returnvalue (Math|Random|RandomInteger _attackarmcount))
  (Development|PrintString (Utilities|String|ToString(Integer) _returnvalue))
  (switch int _returnvalue
    (:0
      (Components|Timeline|PlayfromStart (Variables|Default|GetRight%20Arm%20Anim)))
    (:1
      (Components|Timeline|PlayfromStart (Variables|Default|GetRight%20Arm%20Anim1)))
    (:2
      (Components|Timeline|PlayfromStart (Variables|Default|GetLeft%20Arm%20Anim1)))
    (:3
      (Components|Timeline|PlayfromStart (Variables|Default|GetLeft%20Arm%20Anim)))))

(fn TwoHanded
  (bind _armright1mesh (Variables|Default|GetarmRight1Mesh))
  (Variables|Default|SetIsTwoHanded true)
  (Variables|Default|SetAttackArmCount 2)
  (Variables|Default|SetAttackCoolDown 0.75)
  (Math|Float|IncrementFloat (Variables|Default|GetAttackDamage)
    (:%20%20
      (Rendering|SetVisibility _armright1mesh true true)
      (Transformation|SetRelativeScale3D _armright1mesh "1.000000,0.700000,1.400000")
      (Transformation|SetRelativeRotation _armright1mesh "20.000000, 0,-45.000000" false false))))

(fn Shielded
  (Variables|Default|SetIsShielded true)
  (Variables|Default|SetBlock 0.15)
  (Variables|Default|SetDefence (+ (Variables|Default|GetDefence) 0.05))
  (Variables|Default|SetMaxHealth (+ (Variables|Default|GetMaxHealth) 1e+01))
  (Rendering|SetVisibility (Variables|Default|GetshieldMesh) true false))

(fn NeedAnotherArm?
  (bind _armleft1mesh (Variables|Default|GetarmLeft1Mesh))
  (Variables|Default|SetIsNeedAnotherArm true)
  (Variables|Default|SetAttackArmCount 3)
  (Variables|Default|SetAttackCoolDown 0.5)
  (Math|Float|IncrementFloat (Variables|Default|GetAttackDamage)
    (:%20%20
      (Rendering|SetVisibility _armleft1mesh true true)
      (Transformation|SetRelativeScale3D _armleft1mesh "1.000000,0.700000,1.400000")
      (Transformation|SetRelativeRotation _armleft1mesh "-20.000000, 0,-45.000000" false false)
      (Transformation|AddRelativeLocation _armleft1mesh "0.000000,-15.000000,30.000000" false false))))

(fn Reflected
  (Variables|Default|SetIsReflected true)
  (Variables|Default|SetBlock 3e+01)
  (Variables|Default|SetDefence (+ (Variables|Default|GetDefence) 0.05))
  (Variables|Default|SetMaxHealth (+ (Variables|Default|GetMaxHealth) 1e+01))
  (Rendering|SetVisibility (Variables|Default|GetshieldMesh1) true false))

(fn Seraphim
  (bind _armleftmesh (Variables|Default|GetarmLeftMesh))
  (Variables|Default|SetIsSeraphim true)
  (Variables|Default|SetAttackArmCount 4)
  (Variables|Default|SetAttackRadius 5e+01)
  (Variables|Default|SetAttackCoolDown 0.2)
  (Variables|Default|SetAttackDamage (+ (Variables|Default|GetAttackDamage) 2.0))
  (Rendering|SetVisibility _armleftmesh true true)
  (Transformation|SetRelativeScale3D _armleftmesh "1.000000,0.700000,1.400000")
  (Transformation|SetRelativeRotation _armleftmesh "40.000000,20.000000,-70.000000" false false)
  (Transformation|AddRelativeLocation _armleftmesh "10.000000,-8.000000,0.000000" false false))

(fn Turtle
  (Variables|Default|SetIsTurtle true)
  (Variables|Default|SetBlock 0.5)
  (Variables|Default|SetDefence (+ (Variables|Default|GetDefence) 0.1))
  (Variables|Default|SetAttackDamage (+ (Variables|Default|GetAttackDamage) 4.0))
  (Rendering|SetVisibility (Variables|Default|GetturtleMesh1) true false))