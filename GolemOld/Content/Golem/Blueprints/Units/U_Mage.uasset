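; Mage unit that can merge with other units and gain skills along three exclusive two-tier branches: Shocking, Energy Field or Projector.
; MageMerge gives the main unit the best group multipliers, destroys the others and fills widget buttons with available skills.
; MageUpgrade applies the selected skill and closes the merge; first-tier skills reveal parts that Tick rotates, second-tier ones only set flags.
; ShootTarget fires projectiles when line of sight is clear.
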(event Custom|Mage%20Merge
  (bind _asplayer_unit (Utilities|Casting|CastToPlayerUnit (Game|Player|GetPlayerPawn 0)))
  (Variables|Default|SetAs%20Player%20Unit _asplayer_unit)
  (Variables|Default|SetButtonholder (Variables|/Game/Golem/UI/MergeMenues/MageMergeMenu.MageMergeMenu_C|GetButtonholder (Variables|/Game/Golem/Blueprints/Units/PlayerUnit.PlayerUnit_C|GetMage%20Widget _asplayer_unit)))
  (if (== self (Variables|/Game/Golem/Blueprints/Units/PlayerUnit.PlayerUnit_C|GetMainMergeUnit (Variables|Default|GetAs%20Player%20Unit)))
    ;[1 1 1] Stat setting
    (for _array_element (Variables|/Game/Golem/Blueprints/Units/PlayerUnit.PlayerUnit_C|GetMergeUnits (Variables|Default|GetAs%20Player%20Unit))
      (if (> (Variables|/Game/Golem/Blueprints/Units/Unit.Unit_C|GetAttackDamageMultiplier _array_element) (Variables|Default|GetAttackDamageMultiplier))
        (Variables|Default|SetAttackDamageMultiplier (Variables|/Game/Golem/Blueprints/Units/Unit.Unit_C|GetAttackDamageMultiplier _array_element))))
    (for _array_element_2 (Variables|/Game/Golem/Blueprints/Units/PlayerUnit.PlayerUnit_C|GetMergeUnits (Variables|Default|GetAs%20Player%20Unit))
      (if (not (> (Variables|/Game/Golem/Blueprints/Units/Unit.Unit_C|GetAttackCoolDownMultiplier _array_element_2) (Variables|Default|GetAttackCoolDownMultiplier)))
        (Variables|Default|SetAttackCoolDownMultiplier (Variables|/Game/Golem/Blueprints/Units/Unit.Unit_C|GetAttackCoolDownMultiplier _array_element_2))))
    (for _array_element_3 (Variables|/Game/Golem/Blueprints/Units/PlayerUnit.PlayerUnit_C|GetMergeUnits (Variables|Default|GetAs%20Player%20Unit))
      (if (> (Variables|/Game/Golem/Blueprints/Units/Unit.Unit_C|GetDefenceMultiplier _array_element_3) (Variables|Default|GetDefenceMultiplier))
        (Variables|Default|SetDefenceMultiplier (Variables|/Game/Golem/Blueprints/Units/Unit.Unit_C|GetDefenceMultiplier _array_element_3))))
    (for _array_element_4 (Variables|/Game/Golem/Blueprints/Units/PlayerUnit.PlayerUnit_C|GetMergeUnits (Variables|Default|GetAs%20Player%20Unit))
      (if (> (Variables|/Game/Golem/Blueprints/Units/Unit.Unit_C|GetMaxHealthMultiplier _array_element_4) (Variables|Default|GetMaxHealthMultiplier))
        (Variables|Default|SetMaxHealthMultiplier (Variables|/Game/Golem/Blueprints/Units/Unit.Unit_C|GetMaxHealthMultiplier _array_element_4))))
    (bind _array_element_5 (Utilities|Array|ForEachLoopwithBreak (Variables|/Game/Golem/Blueprints/Units/PlayerUnit.PlayerUnit_C|GetMergeUnits (Variables|Default|GetAs%20Player%20Unit)))
      (:LoopBody
        (if (not (== _array_element_5 (Variables|/Game/Golem/Blueprints/Units/PlayerUnit.PlayerUnit_C|GetMainMergeUnit (Variables|Default|GetAs%20Player%20Unit))))
          (Actor|DestroyActor _array_element_5)))
      (:Completed
        ;[1 1 1] Adding skills (ints) to array
        (Utilities|Array|Clear (Variables|Default|GetAwailable%20skills))
        (for _index (range 0 2)
          (switch int _index
            (:0
              ;[1 1 1] Shocking
              (if (not (or (Variables|Default|GetHasEnergyField) (Variables|Default|GetHasProjector)))
                (if (Variables|Default|GetHasShocking)
                  ;[1 1 1] Quickfire
                  (if (Variables|Default|GetHasShocking)
                    (if (not (Variables|Default|GetHasAftershock))
                      (Utilities|Array|Add (Variables|Default|GetAwailable%20skills) (+ 0 3))))
                  (else
                    (Utilities|Array|Add (Variables|Default|GetAwailable%20skills) (+ 0 0))))))
            (:1
              ;[1 1 1] Energy Field
              (if (not (or (Variables|Default|GetHasShocking) (Variables|Default|GetHasProjector)))
                (if (Variables|Default|GetHasEnergyField)
                  ;[1 1 1] Salvo
                  (if (Variables|Default|GetHasEnergyField)
                    (if (not (Variables|Default|GetHasFieldOfInfluence))
                      (Utilities|Array|Add (Variables|Default|GetAwailable%20skills) (+ 0 4))))
                  (else
                    (Utilities|Array|Add (Variables|Default|GetAwailable%20skills) (+ 0 1))))))
            (:2
              ;[1 1 1] Projector
              (if (not (or (Variables|Default|GetHasShocking) (Variables|Default|GetHasEnergyField)))
                (if (Variables|Default|GetHasProjector)
                  ;[1 1 1] Salvo
                  (if (Variables|Default|GetHasProjector)
                    (if (not (Variables|Default|GetHasForceField))
                      (Utilities|Array|Add (Variables|Default|GetAwailable%20skills) (+ 0 5))))
                  (else
                    (Utilities|Array|Add (Variables|Default|GetAwailable%20skills) (+ 0 2))))))))
        ;[1 1 1] Creating buttons
        (for (_array_element_6 _array_index) (Variables|Default|GetAwailable%20skills)
          (for (_array_element_7 _array_index_2) (Class|PanelWidget|GetAllChildren (Variables|Default|GetButtonholder))
            (if (or (== (* _array_index 2) _array_index_2) (== (+ (* _array_index 2) 1) _array_index_2))
              (bind _astext (Utilities|Casting|CastToTextBlock _array_element_7)
                (:then
                  (Widget|SetVisibility _array_element_7 "Visible")
                  ;[1 1 1] Setting Text description
                  (switch int _array_element_6
                    (:0
                      (Rendering|Components|TextRender|SetText _astext "Shocking"))
                    (:1
                      (Rendering|Components|TextRender|SetText _astext "Energy Shield"))
                    (:2
                      (Rendering|Components|TextRender|SetText _astext "Projector"))
                    (:3
                      (Rendering|Components|TextRender|SetText _astext "Aftershock"))
                    (:4
                      (Rendering|Components|TextRender|SetText _astext "Field Of Influence"))
                    (:5
                      (Rendering|Components|TextRender|SetText _astext "Force Field"))))
                (:CastFailed
                  (Widget|SetVisibility _array_element_7 "Visible"))))))))))

(event Custom|MageUpgrade
  (bind _as_player_unit (Variables|Default|GetAs%20Player%20Unit))
  (bind _mainmergeunit (Variables|/Game/Golem/Blueprints/Units/PlayerUnit.PlayerUnit_C|GetMainMergeUnit _as_player_unit))
  ;[1 1 1] Checking Array and setting Corresponding Boolean (skill) to true
  (bind (_array_element _array_index) (Utilities|Array|ForEachLoopwithBreak (Variables|Default|GetAwailable%20skills) :!label _label)
    (:LoopBody
      (if (== _array_index (Variables|Default|GetASpos))
        (switch int _array_element
          (:0
            (CallFunction|Shocking))
          (:1
            (CallFunction|EnergyField))
          (:2
            (CallFunction|Projector))
          (:3
            (CallFunction|Aftershock))
          (:4
            (CallFunction|FieldOfInfluence))
          (:5
            (CallFunction|ForceField)))
        (Variables|Default|SetASpos 0)
        (Variables|/Game/Golem/Blueprints/Units/Unit.Unit_C|SetMerges _mainmergeunit (+ (Variables|/Game/Golem/Blueprints/Units/Unit.Unit_C|GetMerges _mainmergeunit) 1))
        (Utilities|Array|Clear (Variables|/Game/Golem/Blueprints/Units/PlayerUnit.PlayerUnit_C|GetMergeUnits _as_player_unit))
        (for _array_element_2 (Class|PanelWidget|GetAllChildren (Variables|Default|GetButtonholder))
          (Widget|SetVisibility _array_element_2 "Collapsed"))
        (Widget|RemovefromParent (Variables|/Game/Golem/Blueprints/Units/PlayerUnit.PlayerUnit_C|GetMage%20Widget _as_player_unit))
        (Default|StopMerge (Variables|/Game/Golem/Blueprints/Units/PlayerUnit.PlayerUnit_C|GetUnitInformation _as_player_unit))
        (goto _label Break)))))

(event EventBeginPlay
  (CallFunction|Init))

(event EventTick
  (params (DeltaSeconds :type Float%20%28single-precision%29))
  (|CallParentFunction DeltaSeconds)
  (Utilities|FlowControl|Sequence
    (:then_0
      (if (> (Variables|Default|GetHealth) 0.0)
        (Utilities|FlowControl|Sequence
          (:then_0
            (if (Variables|Default|GetHasShocking)
              (CallFunction|ElectricAnim)))
          (:then_1
            (if (Variables|Default|GetHasEnergyField)
              (CallFunction|AOEAnim)))
          (:then_2
            (if (Variables|Default|GetHasProjector)
              (CallFunction|ShieldAnim))))))))

(event EventAttack
  (if (> (Variables|Default|GetHealth) 0.0)
    (if (> (Variables|Default|GetTimeSinceLastAttack) (Variables|Default|GetAttackCoolDown))
      (Variables|Default|SetTimeSinceLastAttack 0.0))))

(fn ConstructionScript
  (|CallParentFunction)
  (Rendering|Material|SetMaterial (Variables|Default|GetheadCrystal) 0 (Variables|Default|GetCrystalMaterial)))

(fn ShootTarget
  (bind _targetactor (Variables|Default|GetTargetActor))
  (bind _shootfromposition (Variables|Default|GetShootFromPosition))
  (bind _returnvalue (Transformation|GetActorLocation _targetactor))
  (bind _returnvalue_2 (Transformation|GetWorldLocation _shootfromposition))
  (bind _returnvalue_3 (+ _returnvalue (Math|Vector|MakeVector 0.0 0.0 1e+01)))
  (Utilities|IsValid self
    (:Is%20Valid
      (Utilities|IsValid _targetactor
        (:Is%20Valid
          (Transformation|SetWorldRotation _shootfromposition (Math|Rotator|FindLookatRotation _returnvalue_2 _returnvalue_3) false false)
          (bind _result (CallFunction|HasLineOfSight _returnvalue_2 _returnvalue_3 (Utilities|Array|MakeArray self _targetactor)))
          (if _result
            (Components|Activation|Activate (Variables|Default|GetParticleSystem_0) true)
            (Game|SpawnActorfromClass "/Game/Golem/Blueprints/Units/UnitProjectile.UnitProjectile_C" (Transformation|GetWorldTransform (Variables|Default|GetShootFromPosition)) "AlwaysSpawn" 0 (Variables|Default|GetProjectileSpeed) 0)))))))

(fn ElectricAnim
  (bind _animrotationspeed (Variables|Default|GetAnimRotationSpeed))
  (Transformation|AddLocalRotation (Variables|Default|GetERing1) (Math|Rotator|MakeRotator 0.0 _animrotationspeed 0.0) false false)
  (Transformation|AddLocalRotation (Variables|Default|GetECrystal3) (Math|Rotator|MakeRotator 0.0 0.0 (* _animrotationspeed -2.0)) false false))

(fn ShieldAnim
  (Transformation|AddLocalRotation (Variables|Default|GetouterRing) (Math|Rotator|MakeRotator 0.0 0.0 (Variables|Default|GetAnimRotationSpeed)) false false))

(fn AOEAnim
  (Transformation|AddLocalRotation (Variables|Default|GetSpinny) (Math|Rotator|MakeRotator 0.0 0.0 (Variables|Default|GetAnimRotationSpeed)) false false))

(fn Shocking
  (Variables|Default|SetHasShocking true)
  (Transformation|SetRelativeLocation (Variables|Default|GetElectric) "0, 0, 0" false false)
  (Rendering|SetVisibility (Variables|Default|GetElectric) true true))

(fn EnergyField
  (Variables|Default|SetHasEnergyField true)
  (Transformation|SetRelativeLocation (Variables|Default|GetAOE) "0, 0, 0" false false)
  (Rendering|SetVisibility (Variables|Default|GetAOE) true true))

(fn Projector
  (Variables|Default|SetHasProjector true)
  (Transformation|SetRelativeLocation (Variables|Default|GetShield) "0, 0, 0" false false)
  (Rendering|SetVisibility (Variables|Default|GetShield) true true))

(fn Aftershock
  (Variables|Default|SetHasAftershock true))

(fn FieldOfInfluence
  (Variables|Default|SetHasFieldOfInfluence true))

(fn ForceField
  (Variables|Default|SetHasForceField true))