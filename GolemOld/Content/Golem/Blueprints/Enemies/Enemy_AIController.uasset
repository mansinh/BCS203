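; AI controller for enemy units that runs EnemyBehaviourTree and feeds it target detection data.
; Each tick, a sphere overlap within the unit's DetectRange feeds FindClosestActor, which picks the nearest Unit or PlayerUnit with non-negative Health, ignoring its Tag input.
; The result sets the TargetDetected and TargetLocation blackboard keys, the unit's TargetActor and the controller's focal point.
; A MoveUnit event provides simple move-to-location navigation.
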(event EventBeginPlay
  (AI|RunBehaviorTree "/Game/Golem/Blueprints/Enemies/EnemyBehaviourTree.EnemyBehaviourTree"))

(event EventMoveUnit
  (params (TargetLocation :type Vector :default "0, 0, 0"))
  (AI|Navigation|SimpleMovetoLocation self TargetLocation))

(event EventTick
  (params (DeltaSeconds :type Float%20%28single-precision%29))
  (bind _blackboard (Variables|Default|GetBlackboard))
  (bind _asenemy_unit (Utilities|Casting|CastToEnemyUnit (Pawn|GetControlledPawn)))
  (bind _outactors (Collision|SphereOverlapActors (Transformation|GetActorLocation _asenemy_unit) (Variables|/Game/Golem/Blueprints/Enemies/EnemyUnit.EnemyUnit_C|GetDetectRange _asenemy_unit) (Utilities|Array|MakeArray "ObjectTypeQuery3") 0 (Utilities|Array|MakeArray _asenemy_unit)))
  (bind _targetactor (CallFunction|FindClosestActor _outactors (Transformation|GetActorLocation _asenemy_unit) (Variables|/Game/Golem/Blueprints/Enemies/EnemyUnit.EnemyUnit_C|GetDetectRange _asenemy_unit) "Player"))
  (AI|Components|Blackboard|SetValueasBool _blackboard (Utilities|Name|MakeLiteralName "TargetDetected") (Utilities|IsValid _targetactor))
  (if (Utilities|IsValid _targetactor)
    (AI|Components|Blackboard|SetValueasVector _blackboard (Utilities|Name|MakeLiteralName "TargetLocation") (Transformation|GetActorLocation _targetactor))
    (bind _output_get (Variables|/Game/Golem/Blueprints/Enemies/EnemyUnit.EnemyUnit_C|SetTargetActor _asenemy_unit _targetactor))
    (AI|SetFocalPoint (Transformation|GetActorLocation _output_get))
    (Utilities|FlowControl|Delay 1.0)))

(fn ConstructionScript)

(fn FindClosestActor
  (params (Actors :type Array%20of%20Actor%20Object%20References) (Position :type Vector) (Range :type Float%20%28single-precision%29) (Tag :type Name))
  (LocalVariables|SetClosestSqDist (* Range Range))
  (LocalVariables|SetClosestActor 0)
  (for _array_element Actors
    (bind _asunit (Utilities|Casting|CastToUnit _array_element)
      (:then
        (if (>= (Variables|/Game/Golem/Blueprints/Units/Unit.Unit_C|GetHealth _asunit) 0.0)
          (if (< (Class|KismetMathLibrary|VectorDistanceSquared (Transformation|GetActorLocation _array_element) Position) (LocalVariables|GetClosestSqDist)) :!label _label
            (LocalVariables|SetClosestSqDist (Class|KismetMathLibrary|VectorDistanceSquared (Transformation|GetActorLocation _array_element) Position))
            (LocalVariables|SetClosestActor _array_element))))
      (:CastFailed
        (bind _asplayer_unit (Utilities|Casting|CastToPlayerUnit _array_element))
        (if (>= (Variables|/Game/Golem/Blueprints/Units/PlayerUnit.PlayerUnit_C|GetHealth _asplayer_unit) 0.0)
          (goto _label)))))
  (return (LocalVariables|GetClosestActor)))