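; Behavior tree task that makes an AI enemy randomly strafe sideways.
; Half the time, it picks a random offset along the pawn's right vector within MaxStrafeDistance, with the goal's Z set to zero.
; A Visibility trace replaces the goal with any hit location before SimpleMoveToLocation starts the move.
; The task always finishes successfully at once, without waiting for arrival.
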(event EventReceiveExecuteAI
  (params (OwnerController :type AI%20Controller%20Object%20Reference) (ControlledPawn :type Pawn%20Object%20Reference))
  (bind _returnvalue (Transformation|GetActorLocation ControlledPawn))
  (bind _returnvalue_2 (Transformation|GetActorRightVector ControlledPawn))
  (bind _returnvalue_3 (Math|Random|RandomFloatinRange -1.0 1.0))
  (bind _maxstrafedistance (Variables|Default|GetMaxStrafeDistance))
  (bind _returnvalue_4 (* _returnvalue_2 _returnvalue_3))
  (bind _returnvalue_5 (* _returnvalue_4 _maxstrafedistance))
  (bind _returnvalue_6 (+ _returnvalue _returnvalue_5))
  (bind (_x _y) (Math|Vector|BreakVector _returnvalue_6))
  (if (< (Math|Random|RandomFloat) 0.5)
    (bind _output_get (Variables|Default|SetStrafeTo (Math|Vector|MakeVector _x _y 0.0)))
    (bind (_outhit _returnvalue_7) (Collision|LineTraceByChannel _returnvalue _output_get "TraceTypeQuery1" false (Utilities|Array|MakeArray ControlledPawn) "None"))
    (if _returnvalue_7
      (bind _output_get_2 (Variables|Default|SetStrafeTo (.Location (Collision|BreakHitResult _outhit)))))
    (AI|Navigation|SimpleMovetoLocation OwnerController _output_get_2)
    (AI|BehaviorTree|FinishExecute true)
    (else
      (AI|BehaviorTree|FinishExecute true))))