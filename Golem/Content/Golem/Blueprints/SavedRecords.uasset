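; SavedRecords is a save object that keeps a sorted list of time records.
; AddRecord walks the Times array to find where the new time belongs and inserts it there, keeping the list ordered from highest to lowest.
; It then saves itself to the "Records" slot.
; The NewDate input is accepted but never used.
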(event Custom|AddRecord
  (params (NewTIme :type Float%20%28single-precision%29) (NewDate :type Float%20%28single-precision%29))
  (bind _times (Variables|Default|GetTimes))
  (Variables|Default|SetcurrentIndex 0)
  (while (and (< (Variables|Default|GetcurrentIndex) (Utilities|Array|Length _times)) (< NewTIme (Utilities|Array|Get(acopy) _times (Variables|Default|GetcurrentIndex))))
    (Math|Integer|IncrementInt (Variables|Default|GetcurrentIndex)))
  (Utilities|Array|Insert (Variables|Default|GetTimes) NewTIme (Variables|Default|GetcurrentIndex))
  (SaveGame|SaveGametoSlot self "Records"))