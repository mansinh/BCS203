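; Corpse actor for the Golem game that can be repaired back into a unit.
; Repair spawns the RepairedUnit class at the corpse's transform, adjusting for collisions but always spawning, and activates the new unit's repair effect.
; The corpse then destroys itself, after a validity check on SpawnedFrom.
; The construction script sets the actor's world Z to its capsule half-height, keeping X and Y.
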(event Custom|Repair
  (CallFunction|SpawnRepaired)
  (Utilities|IsValid (Variables|Default|GetSpawnedFrom)
    (:Is%20Valid
      (Actor|DestroyActor))
    (:Is%20Not%20Valid
      _))
  (Actor|DestroyActor))

(fn ConstructionScript
  (bind _returnvalue (Transformation|GetActorLocation))
  (Transformation|SetActorLocation (Math|Vector|MakeVector (.x _returnvalue) (.y _returnvalue) (Variables|/Script/Engine.CapsuleComponent|GetCapsuleHalfHeight (Variables|Collision|GetCapsuleComponent))) false false))

(fn SpawnRepaired
  (Development|PrintString "SPAWN")
  (bind _returnvalue (Game|SpawnActorfromClass (Variables|Default|GetRepairedUnit) (Transformation|GetActorTransform) "AdjustIfPossibleButAlwaysSpawn" 0 8e+02 0 0))
  (Components|Activation|Activate (Variables|/Game/Golem/Blueprints/Units/Unit.Unit_C|GetRepairEffect _returnvalue) true))