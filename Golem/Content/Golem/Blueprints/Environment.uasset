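; Environment actor that scatters random corpse actors around the player when play begins.
; On BeginPlay it spawns CorpseCount actors picked from CorpseTypes, always spawning despite collisions, and makes their meshes visible.
; RandomTransform offsets each from player pawn 0 at the same height with random yaw.
; X and Y draw independent angles and distances, so the scatter is not a uniform disc and can exceed SpawnRadius diagonally.
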(event EventBeginPlay
  (bind _corpsetypes (Variables|Default|GetCorpseTypes))
  (for _index (range 0 (Variables|Default|GetCorpseCount))
    (bind _returnvalue (CallFunction|RandomTransform (Variables|Default|GetSpawnRadius)))
    (bind _returnvalue_2 (Game|SpawnActorfromClass (Utilities|Array|Get(acopy) _corpsetypes (Math|Float|Truncate (* (Utilities|Array|Length _corpsetypes) (Math|Random|RandomFloat)))) _returnvalue "AlwaysSpawn" 0 0))
    (Rendering|SetVisibility (Variables|/Game/Golem/Blueprints/Corpses/Corpse.Corpse_C|GetMeshes _returnvalue_2) true true)))

(event Collision|EventActorBeginOverlap
  (params (OtherActor :type Actor%20Object%20Reference)))

(event EventTick
  (params (DeltaSeconds :type Float%20%28single-precision%29)))

(fn ConstructionScript)

(fn RandomTransform
  (params (Radius :type Float%20%28single-precision%29))
  (bind _returnvalue (Math|Random|RandomFloatinRange 0.0 3.6e+02))
  (bind _returnvalue_2 (Math|Random|RandomFloat))
  (bind _returnvalue_3 (* Radius _returnvalue_2))
  (return (Math|Transform|MakeTransform (+ (Math|Vector|MakeVector (* (Math|Trig|Cos(Degrees) _returnvalue) _returnvalue_3) (* (Math|Trig|Sin(Degrees) _returnvalue) _returnvalue_3) 0.0) (Transformation|GetActorLocation (Game|Player|GetPlayerPawn 0))) (Math|Rotator|MakeRotator 0.0 0.0 (Math|Random|RandomFloatinRange 0.0 3.6e+02)))))