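; AI controller for Units that runs their behavior tree and feeds its blackboard with a move target and combat state.
; Each tick the move target becomes the unit's Anchor, offset from the player's position while in control range.
; A sphere overlap picks the nearest "Enemy"-tagged pawn, setting detection and attack-range flags.
; The unit faces that enemy, or otherwise looks along the player body's forward direction.
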(event EventBeginPlay
  (AI|RunBehaviorTree "/Game/Golem/Blueprints/Units/UnitBehaviourTree.UnitBehaviourTree"))

(event EventMoveUnit
  (params (TargetLocation :type Vector :default "0, 0, 0"))
  (AI|Navigation|SimpleMovetoLocation self TargetLocation))

(event EventTick
  (params (DeltaSeconds :type Float%20%28single-precision%29))
  (bind _asunit (Utilities|Casting|CastToUnit (Pawn|GetControlledPawn)))
  (Variables|Default|SetControlledPawn _asunit)
  (Utilities|FlowControl|Sequence
    (:then_0
      (CallFunction|GetMoveTarget))
    (:then_1
      (bind _outactors (Collision|SphereOverlapActors (Transformation|GetActorLocation (Variables|Default|GetControlledPawn)) (Variables|/Game/Golem/Blueprints/Units/Unit.Unit_C|GetDetectRange (Variables|Default|GetControlledPawn)) (Utilities|Array|MakeArray "ObjectTypeQuery3") 0 (Utilities|Array|MakeArray (Variables|Default|GetControlledPawn))))
      (bind _targetactor (CallFunction|FindClosestActor _outactors (Transformation|GetActorLocation (Variables|Default|GetControlledPawn)) (Variables|/Game/Golem/Blueprints/Units/Unit.Unit_C|GetDetectRange (Variables|Default|GetControlledPawn))))
      (AI|Components|Blackboard|SetValueasBool (Variables|Default|GetBlackboard) (Utilities|Name|MakeLiteralName "TargetDetected") (Utilities|IsValid _targetactor))
      (if (Utilities|IsValid _targetactor)
        (bind _output_get (Variables|/Game/Golem/Blueprints/Units/Unit.Unit_C|SetTargetActor (Variables|Default|GetControlledPawn) _targetactor))
        (AI|SetFocalPoint (Math|Vector|MakeVector (.x (Transformation|GetActorLocation _output_get)) (.y (Transformation|GetActorLocation _output_get)) 1e+02))
        (AI|Components|Blackboard|SetValueasBool (Variables|Default|GetBlackboard) (Utilities|Name|MakeLiteralName "InAttackRange") (< (Math|Vector|Distance(Vector) (Transformation|GetActorLocation _output_get) (Transformation|GetActorLocation (Variables|Default|GetControlledPawn))) (Variables|/Game/Golem/Blueprints/Units/Unit.Unit_C|GetAttackRange (Variables|Default|GetControlledPawn))))
        (else
          (AI|Components|Blackboard|SetValueasBool (Variables|Default|GetBlackboard) (Utilities|Name|MakeLiteralName "InAttackRange") false)
          (bind _asplayer_unit (Utilities|Casting|CastToPlayerUnit (Game|Player|GetPlayerPawn 0)))
          (AI|SetFocalPoint (+ (Transformation|GetActorLocation (Game|Player|GetPlayerPawn 0)) (* (Math|Vector|GetForwardVector (Variables|/Game/Golem/Blueprints/Units/PlayerUnit.PlayerUnit_C|GetBody _asplayer_unit)) 1e+03))))))))

(fn ConstructionScript)

(fn FindClosestActor
  (params (Actors :type Array%20of%20Actor%20Object%20References) (Position :type Vector) (Range :type Float%20%28single-precision%29))
  (LocalVariables|SetClosestSqDist (* Range Range))
  (LocalVariables|SetClosestActor 0)
  (for _array_element Actors
    (if (Actor|ActorHasTag _array_element "Enemy")
      (if (< (Class|KismetMathLibrary|VectorDistanceSquared (Transformation|GetActorLocation _array_element) Position) (LocalVariables|GetClosestSqDist))
        (LocalVariables|SetClosestSqDist (Class|KismetMathLibrary|VectorDistanceSquared (Transformation|GetActorLocation _array_element) Position))
        (LocalVariables|SetClosestActor _array_element))))
  (return (LocalVariables|GetClosestActor)))

(fn GetMoveTarget
  (bind _returnvalue (Utilities|Name|MakeLiteralName "TargetLocation"))
  (bind _controlledpawn (Variables|Default|GetControlledPawn))
  (bind _blackboard (Variables|Default|GetBlackboard))
  (if (Variables|/Game/Golem/Blueprints/Units/Unit.Unit_C|GetInControlRange _controlledpawn)
    (AI|Components|Blackboard|SetValueasVector _blackboard _returnvalue (+ (Variables|/Game/Golem/Blueprints/Units/Unit.Unit_C|GetAnchor _controlledpawn) (Transformation|GetActorLocation (Game|Player|GetPlayerPawn 0))))
    (else
      (AI|Components|Blackboard|SetValueasVector _blackboard _returnvalue (Variables|/Game/Golem/Blueprints/Units/Unit.Unit_C|GetAnchor _controlledpawn)))))