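; Piercing unit projectile that can pass through several targets, with its launch speed set from Speed in the construction script.
; Each overlap end with a valid actor decrements Hits; Enemy targets receive attack damage with zero knockback, while E_Sentinel skips the damage call.
; Both target types activate Hit, and exhausted Hits hides the mesh before a delayed destroy.
; Any other actor destroys the projectile immediately.
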(event Collision|EventActorEndOverlap
  (params (OtherActor :type Actor%20Object%20Reference))
  (Utilities|IsValid OtherActor
    (:Is%20Valid
      (Math|Integer|DecrementInt (Variables|Default|GetHits)
        (:%20%20
          (Utilities|Casting|CastToE_Sentinel OtherActor
            (:then
              (Components|Activation|Activate (Variables|Default|GetHit) true :!label _label)
              (if (<= (Variables|Default|GetHits) 0)
                (Rendering|SetVisibility (Variables|Default|GetProjectileMesh) false false)
                (Utilities|FlowControl|Delay 2.0)
                (Actor|DestroyActor :!label _label_2)))
            (:CastFailed
              (bind _asenemy (Utilities|Casting|CastToEnemy OtherActor)
                (:then
                  (Class|GolemInterface|Attacked(Message) _asenemy (Variables|Default|GetAttackDamage) "0, 0, 0")
                  (goto _label))
                (:CastFailed
                  (goto _label_2))))))))))

(fn ConstructionScript
  (Variables|/Script/Engine.ProjectileMovementComponent|SetInitialSpeed (Variables|Default|GetProjectileMovement) (Variables|Default|GetSpeed)))