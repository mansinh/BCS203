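; Ranged player unit for a merge-and-upgrade game that attacks its target with projectiles or a beam when it has line of sight.
; RangedMerge takes the best multipliers from the merged units and shows buttons for skills unlocked along a prerequisite tree.
; RangedUpgrade applies the chosen skill's flag or cooldown cut.
; Attack uses those flags to pick single shots, random-yaw spreads, piercing rounds or a sphere-trace beam.
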(event Custom|Ranged%20Merge
  (bind _asplayer_unit (Utilities|Casting|CastToPlayerUnit (Game|Player|GetPlayerPawn 0)))
  (Variables|Default|SetAs%20Player%20Unit _asplayer_unit)
  (Variables|Default|SetButtonholder (Variables|/Game/Golem/UI/RangedMergeMenu.RangedMergeMenu_C|GetButtonholder (Variables|/Game/Golem/Blueprints/Units/PlayerUnit.PlayerUnit_C|GetSkill%20widget _asplayer_unit)))
  ;[1 1 1] Stat setting
  (for _array_element (Variables|/Game/Golem/Blueprints/Units/PlayerUnit.PlayerUnit_C|GetMergeUnits (Variables|Default|GetAs%20Player%20Unit))
    (if (> (Variables|/Game/Golem/Blueprints/Units/Unit.Unit_C|GetAttackDamageMultiplier _array_element) (Variables|Default|GetAttackDamageMultiplier))
      (Variables|Default|SetAttackDamageMultiplier (Variables|/Game/Golem/Blueprints/Units/Unit.Unit_C|GetAttackDamageMultiplier _array_element))))
  (for _array_element_2 (Variables|/Game/Golem/Blueprints/Units/PlayerUnit.PlayerUnit_C|GetMergeUnits (Variables|Default|GetAs%20Player%20Unit))
    (if (> (Variables|/Game/Golem/Blueprints/Units/Unit.Unit_C|GetAttackCoolDownMultiplier _array_element_2) (Variables|Default|GetAttackCoolDownMultiplier))
      (Variables|Default|SetAttackCoolDownMultiplier (Variables|/Game/Golem/Blueprints/Units/Unit.Unit_C|GetAttackCoolDownMultiplier _array_element_2))))
  (for _array_element_3 (Variables|/Game/Golem/Blueprints/Units/PlayerUnit.PlayerUnit_C|GetMergeUnits (Variables|Default|GetAs%20Player%20Unit))
    (if (> (Variables|/Game/Golem/Blueprints/Units/Unit.Unit_C|GetDefenceMultiplier _array_element_3) (Variables|Default|GetDefenceMultiplier))
      (Variables|Default|SetDefenceMultiplier (Variables|/Game/Golem/Blueprints/Units/Unit.Unit_C|GetDefenceMultiplier _array_element_3))))
  (for _array_element_4 (Variables|/Game/Golem/Blueprints/Units/PlayerUnit.PlayerUnit_C|GetMergeUnits (Variables|Default|GetAs%20Player%20Unit))
    (if (> (Variables|/Game/Golem/Blueprints/Units/Unit.Unit_C|GetMaxHealthMultiplier _array_element_4) (Variables|Default|GetMaxHealthMultiplier))
      (Variables|Default|SetMaxHealthMultiplier (Variables|/Game/Golem/Blueprints/Units/Unit.Unit_C|GetMaxHealthMultiplier _array_element_4))))
  (bind (_array_element_5 _array_index) (Utilities|Array|ForEachLoopwithBreak (Variables|/Game/Golem/Blueprints/Units/PlayerUnit.PlayerUnit_C|GetMergeUnits (Variables|Default|GetAs%20Player%20Unit)))
    (:LoopBody
      (if (!= _array_index 0)
        _))
    (:Completed
      ;[1 1 1] Adding skills (ints) to array
      (if (< (Variables|Default|Getmerges) 3)
        (Utilities|Array|Clear (Variables|Default|GetAwailable%20skills))
        (for _index (range 0 6)
          (switch int _index
            (:0
              ;[1 1 1] Quickfire
              (if (not (Variables|Default|GetHasQuickfire))
                (Utilities|Array|Add (Variables|Default|GetAwailable%20skills) (+ 0 0))))
            (:1
              ;[1 1 1] Spreadfire
              (if (not (Variables|Default|GetHasSpreadfire))
                (Utilities|Array|Add (Variables|Default|GetAwailable%20skills) (+ 0 1))))
            (:2
              ;[1 1 1] Pierce
              (if (not (Variables|Default|GetHasPiercing))
                (Utilities|Array|Add (Variables|Default|GetAwailable%20skills) (+ 0 2))))
            (:3
              ;[1 1 1] Quickfire
              (if (Variables|Default|GetHasQuickfire)
                (if (not (Variables|Default|GetHasRapidfire))
                  (Utilities|Array|Add (Variables|Default|GetAwailable%20skills) (+ 0 3)))))
            (:4
              ;[1 1 1] Salvo
              (if (Variables|Default|GetHasSpreadfire)
                (if (not (Variables|Default|GetHasSalvo))
                  (Utilities|Array|Add (Variables|Default|GetAwailable%20skills) (+ 0 4)))))
            (:5
              ;[1 1 1] Comment
              (if (or (Variables|Default|GetHasRapidfire) (and (Variables|Default|GetHasQuickfire) (Variables|Default|GetHasPiercing)))
                (if (not (Variables|Default|GetHasChanneledLight))
                  (Utilities|Array|Add (Variables|Default|GetAwailable%20skills) (+ 0 5)))))
            (:6
              ;[1 1 1] Comment
              (if (or (Variables|Default|GetHasSalvo) (and (Variables|Default|GetHasSpreadfire) (Variables|Default|GetHasPiercing)))
                (if (not (Variables|Default|GetHasArcOfLight))
                  (Utilities|Array|Add (Variables|Default|GetAwailable%20skills) (+ 0 6)))))))
        ;[1 1 1] Creating buttons
        (for (_array_element_6 _array_index_2) (Variables|Default|GetAwailable%20skills)
          (for (_array_element_7 _array_index_3) (Class|PanelWidget|GetAllChildren (Variables|Default|GetButtonholder))
            (if (or (== (* _array_index_2 2) _array_index_3) (== (+ (* _array_index_2 2) 1) _array_index_3))
              (bind _astext (Utilities|Casting|CastToTextBlock _array_element_7)
                (:then
                  (Widget|SetVisibility _array_element_7 "Visible")
                  ;[1 1 1] Setting Text description
                  (switch int _array_element_6
                    (:0
                      (Rendering|Components|TextRender|SetText _astext "Quickfire"))
                    (:1
                      (Rendering|Components|TextRender|SetText _astext "Spreadfire"))
                    (:2
                      (Rendering|Components|TextRender|SetText _astext "Pierce"))
                    (:3
                      (Rendering|Components|TextRender|SetText _astext "Rapidfire"))
                    (:4
                      (Rendering|Components|TextRender|SetText _astext "Salvo"))
                    (:5
                      (Rendering|Components|TextRender|SetText _astext "Channeled light"))
                    (:6
                      (Rendering|Components|TextRender|SetText _astext "Arc of light"))))
                (:CastFailed
                  (Widget|SetVisibility _array_element_7 "Visible"))))))))))

(event Custom|RangedUpgrade
  (bind _as_player_unit (Variables|Default|GetAs%20Player%20Unit))
  ;[1 1 1] Checking Array and setting Corresponding Boolean (skill) to true
  (bind (_array_element _array_index) (Utilities|Array|ForEachLoopwithBreak (Variables|Default|GetAwailable%20skills) :!label _label)
    (:LoopBody
      (if (== _array_index (Variables|Default|GetASpos))
        (switch int _array_element
          (:0
            (CallFunction|Quickfire))
          (:1
            (CallFunction|Spreadfire))
          (:2
            (CallFunction|Pierce))
          (:3
            (CallFunction|RapidFire))
          (:4
            (CallFunction|Salvo))
          (:5
            (CallFunction|ChanneledLight))
          (:6
            (CallFunction|ArcOfLight)))
        (Variables|Default|SetASpos 0)
        (Utilities|Array|Clear (Variables|/Game/Golem/Blueprints/Units/PlayerUnit.PlayerUnit_C|GetMergeUnits _as_player_unit))
        (for _array_element_2 (Class|PanelWidget|GetAllChildren (Variables|Default|GetButtonholder))
          (Widget|SetVisibility _array_element_2 "Collapsed"))
        (Widget|RemovefromParent (Variables|/Game/Golem/Blueprints/Units/PlayerUnit.PlayerUnit_C|GetSkill%20widget _as_player_unit))
        (goto _label Break)))))

(event EventBeginPlay
  (CallFunction|Init))

(event Collision|EventActorBeginOverlap
  (params (OtherActor :type Actor%20Object%20Reference)))

(event EventTick
  (params (DeltaSeconds :type Float%20%28single-precision%29))
  (|CallParentFunction DeltaSeconds))

(event EventAttack
  (if (> (Variables|Default|GetHealth) 0.0)
    (if (> (Variables|Default|GetTimeSinceLastAttack) (* (Variables|Default|GetAttackCoolDown) (Variables|Default|GetAttackCoolDownMultiplier)))
      (Variables|Default|SetTimeSinceLastAttack 0.0)
      (if (Variables|Default|GetHasChanneledLight)
        (CallFunction|ShootBeam)
        (Utilities|FlowControl|Delay 0.2)
        (Rendering|SetVisibility (Variables|Default|Getbeam) false false)
        (elif (Variables|Default|GetHasArcOfLight)
          (CallFunction|ShootTargetSpread 10)
          (elif (Variables|Default|GetHasSalvo)
            (CallFunction|ShootTargetSpread 5)
            (elif (Variables|Default|GetHasSpreadfire)
              (CallFunction|ShootTargetSpread 3)
              (else
                (CallFunction|ShootTarget)))))))))

(fn ConstructionScript
  (|CallParentFunction)
  (Rendering|Material|SetMaterial (Variables|Default|Geteye) 0 (Variables|Default|GetCrystalMaterial)))

(fn ShootTarget
  (bind _shootfromposition (Variables|Default|GetShootFromPosition))
  (bind _targetactor (Variables|Default|GetTargetActor))
  (bind _projectilespeed (Variables|Default|GetProjectileSpeed))
  (bind _shootfromposition_2 (Variables|Default|GetShootFromPosition))
  (bind _returnvalue (Transformation|GetActorLocation _targetactor))
  (bind _returnvalue_2 (Transformation|GetWorldLocation _shootfromposition_2))
  (bind _returnvalue_3 (Transformation|GetWorldTransform _shootfromposition))
  (bind _returnvalue_4 (+ _returnvalue (Math|Vector|MakeVector 0.0 0.0 1e+01)))
  (Utilities|IsValid self
    (:Is%20Valid
      (Utilities|IsValid _targetactor
        (:Is%20Valid
          (Transformation|SetWorldRotation _shootfromposition_2 (Math|Rotator|FindLookatRotation _returnvalue_2 _returnvalue_4) false false)
          (bind _result (CallFunction|HasLineOfSight _returnvalue_2 _returnvalue_4 (Utilities|Array|MakeArray self _targetactor)))
          (if _result
            (Components|Activation|Activate (Variables|Default|GetParticleSystem_0) true)
            (if (Variables|Default|GetHasPiercing)
              (bind _returnvalue_5 (Game|SpawnActorfromClass "/Game/Golem/Blueprints/Units/UnitProjectile_Piercing.UnitProjectile_Piercing_C" _returnvalue_3 "AlwaysSpawn" 0 _projectilespeed 0))
              (Utilities|IsValid _returnvalue_5
                (:Is%20Valid
                  (Variables|/Game/Golem/Blueprints/Units/UnitProjectile_Piercing.UnitProjectile_Piercing_C|SetAttackDamage _returnvalue_5 (* (Variables|Default|GetAttackDamage) (Variables|Default|GetAttackDamageMultiplier)))))
              (else
                (bind _returnvalue_6 (Game|SpawnActorfromClass "/Game/Golem/Blueprints/Units/UnitProjectile.UnitProjectile_C" _returnvalue_3 "AlwaysSpawn" 0 _projectilespeed 0))
                (Utilities|IsValid _returnvalue_6
                  (:Is%20Valid
                    (Variables|/Game/Golem/Blueprints/Units/UnitProjectile.UnitProjectile_C|SetAttackDamage _returnvalue_6 (* (Variables|Default|GetAttackDamage) (Variables|Default|GetAttackDamageMultiplier)))))))))))))

(fn Pierce
  (Variables|Default|SetHasPiercing true))

(fn Quickfire
  (Variables|Default|SetHasQuickfire true)
  (Variables|Default|SetAttackCoolDown (/ (Variables|Default|GetAttackCoolDown) 3.0)))

(fn Spreadfire
  (Variables|Default|SetHasSpreadfire true))

(fn RapidFire
  (Variables|Default|SetHasRapidfire true)
  (Variables|Default|SetAttackCoolDown (/ (Variables|Default|GetAttackCoolDown) 2.0)))

(fn Salvo
  (Variables|Default|SetHasSalvo true))

(fn ChanneledLight
  (Variables|Default|SetHasChanneledLight true))

(fn ArcOfLight
  (Variables|Default|SetHasArcOfLight true))

(fn ShootTargetSpread
  (params (ProjectileCount :type Integer))
  (bind _returnvalue (Math|Random|RandomFloatinRange -1e+01 1e+01))
  (bind _shootfromposition (Variables|Default|GetShootFromPosition))
  (bind _targetactor (Variables|Default|GetTargetActor))
  (bind _projectilespeed (Variables|Default|GetProjectileSpeed))
  (bind _shootfromposition_2 (Variables|Default|GetShootFromPosition))
  (bind _returnvalue_2 (Transformation|GetActorLocation _targetactor))
  (bind _returnvalue_3 (Transformation|GetWorldLocation _shootfromposition_2))
  (bind _returnvalue_4 (Transformation|GetWorldTransform _shootfromposition))
  (bind _returnvalue_5 (+ _returnvalue_2 (Math|Vector|MakeVector 0.0 0.0 1e+01)))
  (bind _returnvalue_6 (+ (.yaw (.rotation _returnvalue_4)) _returnvalue))
  (bind _returnvalue_7 (Math|Rotator|MakeRotator (.roll (.rotation _returnvalue_4)) (.pitch (.rotation _returnvalue_4)) _returnvalue_6))
  (bind _returnvalue_8 (Math|Transform|MakeTransform (.location _returnvalue_4) _returnvalue_7 (.scale _returnvalue_4)))
  (Utilities|IsValid self
    (:Is%20Valid
      (Utilities|IsValid _targetactor
        (:Is%20Valid
          (Transformation|SetWorldRotation _shootfromposition_2 (Math|Rotator|FindLookatRotation _returnvalue_3 _returnvalue_5) false false)
          (bind _result (CallFunction|HasLineOfSight _returnvalue_3 _returnvalue_5 (Utilities|Array|MakeArray self _targetactor)))
          (if _result
            (Components|Activation|Activate (Variables|Default|GetParticleSystem_0) true)
            (for _index (range 1 ProjectileCount)
              (if (or (Variables|Default|GetHasPiercing) (Variables|Default|GetHasArcOfLight))
                (bind _returnvalue_9 (Game|SpawnActorfromClass "/Game/Golem/Blueprints/Units/UnitProjectile_Piercing.UnitProjectile_Piercing_C" _returnvalue_8 "AlwaysSpawn" 0 _projectilespeed 0))
                (Utilities|IsValid _returnvalue_9
                  (:Is%20Valid
                    (Variables|/Game/Golem/Blueprints/Units/UnitProjectile_Piercing.UnitProjectile_Piercing_C|SetAttackDamage _returnvalue_9 (* (Variables|Default|GetAttackDamage) (Variables|Default|GetAttackDamageMultiplier)))))
                (else
                  (bind _returnvalue_10 (Game|SpawnActorfromClass "/Game/Golem/Blueprints/Units/UnitProjectile.UnitProjectile_C" _returnvalue_8 "AlwaysSpawn" 0 _projectilespeed 0))
                  (Utilities|IsValid _returnvalue_10
                    (:Is%20Valid
                      (Variables|/Game/Golem/Blueprints/Units/UnitProjectile.UnitProjectile_C|SetAttackDamage _returnvalue_10 (* (Variables|Default|GetAttackDamage) (Variables|Default|GetAttackDamageMultiplier))))))))))))))

(fn ShootBeam
  (bind _returnvalue (Transformation|GetActorForwardVector))
  (bind _returnvalue_2 (Transformation|GetActorLocation))
  (bind _targetactor (Variables|Default|GetTargetActor))
  (Utilities|IsValid self
    (:Is%20Valid
      (Utilities|IsValid _targetactor
        (:Is%20Valid
          (bind _result (CallFunction|HasLineOfSight (Transformation|GetWorldLocation (Variables|Default|GetShootFromPosition)) (+ (Transformation|GetActorLocation _targetactor) (Math|Vector|MakeVector 0.0 0.0 1e+01)) (Utilities|Array|MakeArray self _targetactor)))
          (if _result
            (Rendering|SetVisibility (Variables|Default|Getbeam) true false)
            (bind _outhits (Collision|MultiSphereTraceByChannel _returnvalue_2 (+ _returnvalue_2 (* _returnvalue 2e+03)) 5e+01 "TraceTypeQuery2" false 0 "None"))
            (for _array_element _outhits
              (bind _asenemy_unit (Utilities|Casting|CastToEnemyUnit (.HitActor (Collision|BreakHitResult _array_element))))
              (Default|Attacked _asenemy_unit (* (Variables|Default|GetAttackDamage) (Variables|Default|GetAttackDamageMultiplier)) (* _returnvalue (Variables|Default|GetKnockback))))))))))