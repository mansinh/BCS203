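; OrbitingCrystal is an actor that spins its CrystalOrbit component to make a crystal orbit on a randomized, slanted path.
; The construction script randomizes rotation direction, speed, slant amount and starting yaw.
; Each Tick, Orbit adds yaw scaled by BaseOrbitSpeed, without delta time, and sets the component's relative height to slant times the sine of that yaw, faking a tilted orbit.
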(event EventBeginPlay)

(event Collision|EventActorBeginOverlap
  (params (OtherActor :type Actor%20Object%20Reference)))

(event EventTick
  (params (DeltaSeconds :type Float%20%28single-precision%29))
  (CallFunction|Orbit))

(fn ConstructionScript
  (bind _returnvalue (Math|Random|RandomFloatinRange 8.0 15.0))
  (if (Math|Random|RandomBool)
    (Variables|Default|SetRotationSpeed (* -1 _returnvalue))
    (else
      (Variables|Default|SetRotationSpeed _returnvalue)))
  (Variables|Default|SetSlant (Math|Random|RandomFloatinRange -5e+01 5e+01))
  (Transformation|SetRelativeRotation (Variables|Default|GetCrystalOrbit) (Math|Rotator|MakeRotator 0.0 0.0 (Math|Random|RandomFloatinRange 0.0 3.6e+02)) false false))

(fn Orbit
  (bind _crystalorbit (Variables|Default|GetCrystalOrbit))
  (Transformation|AddRelativeRotation _crystalorbit (Math|Rotator|MakeRotator 0.0 0.0 (* (Variables|Default|GetRotationSpeed) (Variables|Default|GetBaseOrbitSpeed))) false false)
  (Transformation|SetRelativeLocation _crystalorbit (Math|Vector|MakeVector 0.0 0.0 (* (Variables|Default|GetSlant) (Math|Trig|Sin(Degrees) (.yaw (Variables|/Script/Engine.SceneComponent|GetRelativeRotation _crystalorbit))))) false false))