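; Melee golem unit that punches with up to four arms and damages targets in front of it.
; Attack checks health and cooldown, plays a random arm's punch timeline, then after a short delay sphere-traces and sends damage and knockback through GolemInterface.
; The construction script applies the crystal material and feeds shared punch curves into the arm timelines.
; Upgrade functions reveal extra arm, shield or turtle meshes and adjust combat stats.
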(event EventBeginPlay
  (CallFunction|Init))

(event EventAttack
  (if (> (Variables|Default|GetHealth) 0.0)
    (if (> (Variables|Default|GetTimeSinceLastAttack) (* (Variables|Default|GetAttackCoolDown) (Variables|Default|GetAttackCoolDownMultiplier)))
      (Variables|Default|SetTimeSinceLastAttack 0.0)
      (CallFunction|AttackAnimation)
      (Utilities|FlowControl|Delay 0.16)
      (CallFunction|MeleeTarget))))

(fn ConstructionScript
  (bind _rightarmanim (Variables|Default|GetrightArmAnim))
  (bind _leftarmanim (Variables|Default|GetleftArmAnim))
  (bind _rightarmanim1 (Variables|Default|GetrightArmAnim1))
  (bind _leftarmanim1 (Variables|Default|GetleftArmAnim1))
  (|CallParentFunction)
  (Rendering|Material|SetMaterial (Variables|Default|GetEye) 0 (Variables|Default|GetCrystalMaterial))
  (Class|TimelineComponent|SetFloatCurve _rightarmanim "/Game/Golem/Blueprints/PunchRotation.PunchRotation" "rotation")
  (Class|TimelineComponent|SetFloatCurve _rightarmanim "/Game/Golem/Blueprints/PunchLocation.PunchLocation" "location")
  (Class|TimelineComponent|SetFloatCurve _leftarmanim "/Game/Golem/Blueprints/PunchRotation.PunchRotation" "rotation")
  (Class|TimelineComponent|SetFloatCurve _leftarmanim "/Game/Golem/Blueprints/PunchLocation.PunchLocation" "location")
  (Class|TimelineComponent|SetFloatCurve _rightarmanim1 "/Game/Golem/Blueprints/PunchRotation.PunchRotation" "rotation")
  (Class|TimelineComponent|SetFloatCurve _rightarmanim1 "/Game/Golem/Blueprints/PunchLocation.PunchLocation" "location")
  (Class|TimelineComponent|SetFloatCurve _leftarmanim1 "/Game/Golem/Blueprints/PunchRotation.PunchRotation" "rotation")
  (Class|TimelineComponent|SetFloatCurve _leftarmanim1 "/Game/Golem/Blueprints/PunchLocation.PunchLocation" "location"))

(fn MeleeTarget
  (bind _meleeattackimpact (Variables|Default|GetMeleeAttackImpact))
  (bind _outhits (Collision|MultiSphereTraceByChannel (Transformation|GetActorLocation) (Transformation|GetWorldLocation (Variables|Default|GetMeleeAttackPosition)) (Variables|Default|GetAttackRadius) "TraceTypeQuery2" false 0 "None"))
  (bind (_array_element _array_index) (Utilities|Array|ForEachLoopwithBreak _outhits :!label _label)
    (:LoopBody
      (if (< _array_index (Variables|Default|GetMaxTargets))
        (if (Utilities|DoesObjectImplementInterface (.HitActor (Collision|BreakHitResult _array_element)) "/Game/Golem/Blueprints/GolemInterface.GolemInterface_C")
          (Transformation|SetWorldLocation _meleeattackimpact (.ImpactPoint (Collision|BreakHitResult _array_element)) false false)
          (Components|Activation|Activate _meleeattackimpact true)
          (bind _knockbackvector (CallFunction|GetKnockback (.HitActor (Collision|BreakHitResult _array_element))))
          (Class|GolemInterface|Attacked(Message) (.HitActor (Collision|BreakHitResult _array_element)) (* (Variables|Default|GetAttackDamage) (Variables|Default|GetAttackDamageMultiplier)) _knockbackvector))
        (else
          (goto _label Break))))))

(fn BlockAttack
  (bind _isblocked (|CallParentFunction))
  (return _isblocked))

(fn AttackAnimation
  (switch int (Math|Random|RandomInteger (Variables|Default|GetAttackArmCount))
    (:0
      (Components|Timeline|PlayfromStart (Variables|Default|GetrightArmAnim)))
    (:1
      (Components|Timeline|PlayfromStart (Variables|Default|GetleftArmAnim)))
    (:2
      (Components|Timeline|PlayfromStart (Variables|Default|GetrightArmAnim1)))
    (:3
      (Components|Timeline|PlayfromStart (Variables|Default|GetleftArmAnim1)))))

(fn TwoHanded
  (Variables|Default|SetIsTwoHanded true)
  (Variables|Default|SetAttackArmCount 2)
  (Variables|Default|SetAttackCoolDown 0.75)
  (Math|Float|IncrementFloat (Variables|Default|GetAttackDamage)
    (:%20%20
      (Rendering|SetVisibility (Variables|Default|GetarmLeftMesh) true false))))

(fn Shielded
  (Variables|Default|SetIsShielded true)
  (Variables|Default|SetBlock 0.15)
  (Variables|Default|SetDefence (+ (Variables|Default|GetDefence) 0.05))
  (Variables|Default|SetMaxHealth (+ (Variables|Default|GetMaxHealth) 1e+01))
  (Rendering|SetVisibility (Variables|Default|GetshieldMesh) true false))

(fn NeedAnotherArm?
  (Variables|Default|SetIsNeedAnotherArm true)
  (Variables|Default|SetAttackArmCount 3)
  (Variables|Default|SetAttackCoolDown 0.5)
  (Math|Float|IncrementFloat (Variables|Default|GetAttackDamage)
    (:%20%20
      (Rendering|SetVisibility (Variables|Default|GetarmRight1Mesh) true false))))

(fn Reflected
  (Variables|Default|SetIsReflected true)
  (Variables|Default|SetBlock 3e+01)
  (Variables|Default|SetDefence (+ (Variables|Default|GetDefence) 0.05))
  (Variables|Default|SetMaxHealth (+ (Variables|Default|GetMaxHealth) 1e+01))
  (Rendering|SetVisibility (Variables|Default|GetshieldMesh1) true false))

(fn Seraphim
  (Variables|Default|SetIsSeraphim true)
  (Variables|Default|SetAttackArmCount 4)
  (Variables|Default|SetAttackRadius 5e+01)
  (Variables|Default|SetAttackCoolDown 0.2)
  (Variables|Default|SetAttackDamage (+ (Variables|Default|GetAttackDamage) 2.0))
  (Rendering|SetVisibility (Variables|Default|GetarmLeft1Mesh) true false))

(fn Turtle
  (Variables|Default|SetIsTurtle true)
  (Variables|Default|SetBlock 0.5)
  (Variables|Default|SetDefence (+ (Variables|Default|GetDefence) 0.1))
  (Variables|Default|SetAttackDamage (+ (Variables|Default|GetAttackDamage) 4.0))
  (Rendering|SetVisibility (Variables|Default|GetturtleMesh) true false))