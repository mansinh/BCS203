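; Defender golem unit that fights with an area stomp, damaging and knocking back nearby enemies through GolemInterface.
; Attack checks health and cooldown, plays the StompAnim timeline, then after a short delay triggers dust and a sphere-overlap hit.
; Upgrade functions set flags and adjust stats or body scale.
; Regrowth periodically repairs the unit on Tick, and Grove extends that repair to nearby Player-tagged allies.
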(event EventBeginPlay
  (CallFunction|Init))

(event Collision|EventActorBeginOverlap
  (params (OtherActor :type Actor%20Object%20Reference)))

(event EventTick
  (params (DeltaSeconds :type Float%20%28single-precision%29))
  (|CallParentFunction DeltaSeconds)
  (Utilities|FlowControl|Sequence
    (:then_0
      (if (Variables|Default|GetHasRegrowth)
        (Variables|Default|SetTimeSinceLastRegen (+ DeltaSeconds (Variables|Default|GetTimeSinceLastRegen)))
        (if (> (Variables|Default|GetTimeSinceLastRegen) 3.0)
          (CallFunction|Repair (Variables|Default|GetRegenAmount))
          (Variables|Default|SetTimeSinceLastRegen 0.0)
          (if (Variables|Default|GetHasGrove)
            (CallFunction|RepairAllies (Variables|Default|GetRegenAmount))))))))

(event EventAttack
  (if (> (Variables|Default|GetHealth) 0.0)
    (if (> (Variables|Default|GetTimeSinceLastAttack) (* (Variables|Default|GetAttackCoolDown) (Variables|Default|GetAttackCoolDownMultiplier)))
      (Variables|Default|SetTimeSinceLastAttack 0.0)
      (Components|Timeline|PlayfromStart (Variables|Default|GetStompAnim))
      (Utilities|FlowControl|Delay 0.6)
      (Components|Activation|Activate (Variables|Default|GetP_StompDust) true)
      (CallFunction|Stomp))))

(fn ConstructionScript
  (bind _stompanim (Variables|Default|GetStompAnim))
  (|CallParentFunction)
  (Rendering|Material|SetMaterial (Variables|Default|Geteye) 0 (Variables|Default|GetCrystalMaterial))
  (Class|TimelineComponent|SetFloatCurve _stompanim "/Game/Golem/Blueprints/Stomp.Stomp" "Location")
  (Class|TimelineComponent|SetFloatCurve _stompanim "/Game/Golem/Blueprints/Stomp_Delayed.Stomp_Delayed" "LocationDelayed"))

(fn ThirstyRock
  (Variables|Default|SetHasThirstyRock true))

(fn Earthquake
  (Variables|Default|SetHasEarthquake true)
  (Variables|Default|SetAttackRange (* (Variables|Default|GetAttackRange) 2.0))
  (Variables|Default|SetAttackDamage (+ (Variables|Default|GetAttackDamage) 5.0)))

(fn Massive
  (Variables|Default|SetHasMassive true)
  (Variables|Default|SetMaxHealth (+ (Variables|Default|GetMaxHealth) 6e+01))
  (Variables|Default|SetDefence (+ (Variables|Default|GetDefence) 0.1))
  (Transformation|SetRelativeScale3D (Variables|Default|GetBody) "1.500000,1.500000,1.100000"))

(fn Grove
  (Variables|Default|SetHasGrove true))

(fn TremblingWeight
  (Variables|Default|SetHasTremblingWeight true)
  (Variables|Default|SetKnockback (* 2 (Variables|Default|GetKnockback)))
  (Variables|Default|SetAttackDamage (+ (Variables|Default|GetAttackDamage) 5.0)))

(fn Chunky
  (Variables|Default|SetHasChunky true)
  (Variables|Default|SetMaxHealth (+ (Variables|Default|GetMaxHealth) 6e+01))
  (Variables|Default|SetDefence (+ (Variables|Default|GetDefence) 0.15))
  (Transformation|SetRelativeScale3D (Variables|Default|GetBody) "1.500000,1.500000, 0"))

(fn WideasAMountain
  (Variables|Default|SetHasWideAsAMountain true)
  (Variables|Default|SetMaxHealth (+ (Variables|Default|GetMaxHealth) 5e+01))
  (Variables|Default|SetDefence (+ (Variables|Default|GetDefence) 0.15))
  (Transformation|SetRelativeScale3D (Variables|Default|GetBody) "1.500000,1.500000, 0"))

(fn Regrowth
  (Variables|Default|SetHasRegrowth true))

(fn LastingImpression
  (Variables|Default|SetHasLastingImpression true)
  (Variables|Default|SetKnockback (* 2 (Variables|Default|GetKnockback)))
  (Variables|Default|SetAttackDamage (+ (Variables|Default|GetAttackDamage) 5.0))
  (Variables|Default|SetAttackCoolDown (/ (Variables|Default|GetAttackCoolDown) 0.75)))

(fn Heal
  (params (Amount :type Float%20%28single-precision%29))
  (Variables|Default|SetHealth (Math|Float|Clamp(Float) (+ (Variables|Default|GetHealth) Amount) 0.0 (Variables|Default|GetMaxHealth)))
  (Components|Activation|Activate (Variables|Default|GetRepairEffect) true))

(fn Stomp
  (Development|PrintString "STOMP")
  (bind _outactors (Collision|SphereOverlapActors (Transformation|GetActorLocation) (Variables|Default|GetAttackRange) (Utilities|Array|MakeArray "ObjectTypeQuery3") 0))
  (for _array_element _outactors
    (if (and (Utilities|DoesObjectImplementInterface _array_element "/Game/Golem/Blueprints/GolemInterface.GolemInterface_C") (Actor|ActorHasTag _array_element "Enemy"))
      (bind _knockbackvector (CallFunction|GetKnockback _array_element))
      (Class|GolemInterface|Attacked(Message) _array_element (* (Variables|Default|GetAttackDamage) (Variables|Default|GetAttackDamageMultiplier)) _knockbackvector))))

(fn RepairAllies
  (params (Amount :type Float%20%28single-precision%29))
  (bind _outactors (Collision|SphereOverlapActors (Transformation|GetActorLocation) 5e+02 (Utilities|Array|MakeArray "ObjectTypeQuery3") 0))
  (for _array_element _outactors
    (if (Actor|ActorHasTag _array_element "Player")
      (Class|GolemInterface|Repair(Message) _array_element Amount))))