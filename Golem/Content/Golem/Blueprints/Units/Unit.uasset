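; Base unit Blueprint that attaches to the player pawn, with health, selection, movement orders, repair and an attack cooldown gate.
; Move orders pass to the controller, and Tick advances the cooldown, tracks movement and draws anchor debug lines while the player builds.
; Incoming hits apply knockback, then a random block roll or defence-reduced damage with a DamageShake timeline.
; Death triggers an explosion effect, spawns a corpse and destroys the unit.
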(event Custom|Repair
  (params (RepairAmount :type Float%20%28single-precision%29))
  (Variables|Default|SetHealth (Math|Float|Clamp(Float) (+ (Variables|Default|GetHealth) RepairAmount) 0.0 (Variables|Default|GetMaxHealth)))
  (Components|Activation|Activate (Variables|Components|GetRepairEffect) true))

(event Custom|Selected
  (CallFunction|OnSelected))

(event EventBeginPlay
  (Variables|Default|SetTimeSinceLastAttack (Variables|Default|GetAttackCoolDown))
  (Variables|/Script/Engine.CharacterMovementComponent|SetMaxWalkSpeed (Variables|Character|GetCharacterMovement) (Variables|Default|GetMovementSpeed))
  (Transformation|AttachActorToActor (Game|Player|GetPlayerPawn 0) "None" "KeepWorld" "KeepWorld" "KeepWorld" true)
  (Variables|Default|SetAnchor (- (Transformation|GetActorLocation self) (Transformation|GetActorLocation (Game|Player|GetPlayerPawn 0))))
  (Class|TimelineComponent|SetFloatCurve (Variables|Default|GetDamageShake) "/Game/Golem/Blueprints/Shake.Shake" "Shake"))

(event EventAttack
  (if (> (Variables|Default|GetHealth) 0.0)
    (if (> (Variables|Default|GetTimeSinceLastAttack) (Variables|Default|GetAttackCoolDown))
      (Variables|Default|SetTimeSinceLastAttack 0.0))))

(event EventTick
  (params (DeltaSeconds :type Float%20%28single-precision%29))
  (bind _returnvalue (Game|Player|GetPlayerPawn 0))
  (bind _self self)
  (bind _anchor (Variables|Default|GetAnchor))
  (bind _returnvalue_2 (Transformation|GetActorLocation _self))
  (if (>= (Variables|Default|GetHealth) 0.0)
    (Variables|Default|SetTimeSinceLastAttack (+ DeltaSeconds (Variables|Default|GetTimeSinceLastAttack)))
    (Utilities|FlowControl|Sequence
      (:then_0
        (bind _asplayer_unit (Utilities|Casting|CastToPlayerUnit _returnvalue))
        (if (Variables|/Game/Golem/Blueprints/Units/PlayerUnit.PlayerUnit_C|GetIsBuilding _asplayer_unit)
          (if (Variables|Default|GetInControlRange)
            (Rendering|Debug|DrawDebugLine _returnvalue_2 (+ (Transformation|GetActorLocation _returnvalue) _anchor) "(R=1.000000,G=1.000000,B=1.000000,A=1.000000)" 0.1 4.0)
            (else
              (Rendering|Debug|DrawDebugLine _returnvalue_2 _anchor "(R=1.000000,G=1.000000,B=1.000000,A=1.000000)" 0.1 4.0)))))
      (:then_1
        (CallFunction|GetDeltaMove DeltaSeconds)))))

(event EventMoveUnit
  (params (TargetLocation :type Vector :default "0, 0, 0"))
  (Class|GolemInterface|MoveUnit(Message) (Pawn|GetController) TargetLocation))

(event EventAttacked
  (params (AttackDamage :type Float%20%28single-precision%29) (AttackKnockback :type Vector :default "0, 0, 0"))
  (Transformation|AddActorWorldOffset AttackKnockback)
  (if (>= (Variables|Default|GetHealth) 0.0)
    (bind _isblocked (CallFunction|Block))
    (if (not _isblocked)
      (CallFunction|TakeDamage AttackDamage)
      (Components|Timeline|PlayfromStart (Variables|Default|GetDamageShake))
      (if (< (Variables|Default|GetHealth) 0.0)
        (CallFunction|Death)))))

(fn ConstructionScript
  (Variables|Default|SetHealth (Variables|Default|GetMaxHealth)))

(fn AngleRange
  (params (AngleIn :type Float%20%28single-precision%29))
  (LocalVariables|SetAngle AngleIn)
  (while (< (LocalVariables|GetAngle) 0.0)
    (LocalVariables|SetAngle (+ (LocalVariables|GetAngle) 3.6e+02)))
  (while (< 3.6e+02 (LocalVariables|GetAngle))
    (LocalVariables|SetAngle (- (LocalVariables|GetAngle) 3.6e+02)))
  (return (LocalVariables|GetAngle)))

(fn Block
  (return (< (* 100 (Math|Random|RandomFloat)) (Variables|Default|GetBlockPercentage))))

(fn Death
  (Components|Activation|Activate (Variables|Components|GetDeathExplosion) true)
  (Game|SpawnActorfromClass (Variables|Default|GetCorpse) (Transformation|GetActorTransform) "Undefined" 0 0)
  (Actor|DestroyActor))

(fn TakeDamage
  (params (damage :type Float%20%28single-precision%29))
  (Variables|Default|SetHealth (- (Variables|Default|GetHealth) (* damage (- 1.0 (/ (Variables|Default|GetDefencePercentage) 1e+02))))))

(fn GetDeltaMove
  (params (deltaSeconds :type Float%20%28single-precision%29))
  (bind _returnvalue (Transformation|GetActorLocation))
  (bind _output_get (Variables|Default|SetDeltaMove (* (* (- _returnvalue (Variables|Default|GetPreviousLocation)) deltaSeconds) 1e+02)))
  (Variables|Default|SetPreviousLocation _returnvalue))

(fn OnSelected
  (if (Variables|Default|GetIsSelected)
    (Variables|Default|SetIsSelected false)
    (Rendering|SetVisibility (Variables|Components|GetSelectCircle) false false)
    (else
      (Variables|Default|SetIsSelected true)
      (Rendering|SetVisibility (Variables|Components|GetSelectCircle) true false))))

(fn GetKnockback
  (params (Target :type Actor%20Object%20Reference))
  (bind _returnvalue (Transformation|GetActorLocation Target))
  (bind _returnvalue_2 (Transformation|GetActorLocation))
  (bind _returnvalue_3 (- _returnvalue _returnvalue_2))
  (return (* (Math|Vector|Normalize (Math|Vector|MakeVector (.x _returnvalue_3) (.y _returnvalue_3) 0.0)) (Variables|Default|GetKnockback))))