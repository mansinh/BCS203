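; FormationGrid is an actor that lays out a square grid of GridCell actors around the player's unit as a formation grid that can be shown or hidden.
; On BeginPlay it snaps to the PlayerUnit pawn, spawns centred cells attached to itself, stores them in Cells and starts hidden.
; Show and Hide events toggle root visibility, propagated to children.
; The player's ControlRadius is cached, but its only check is never run.
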(event Custom|Hide
  (Rendering|SetVisibility (Variables|Default|GetDefaultSceneRoot) false true))

(event Custom|Show
  (Rendering|SetVisibility (Variables|Default|GetDefaultSceneRoot) true true))

(event EventBeginPlay
  (bind _gridsize (Variables|Default|GetGridSize))
  (bind _returnvalue (/ _gridsize 2))
  (bind _asplayer_unit (Utilities|Casting|CastToPlayerUnit (Game|Player|GetPlayerPawn 0)))
  (bind _output_get (Variables|Default|SetPlayer _asplayer_unit))
  (Variables|Default|SetControlRadius (Variables|/Game/Golem/Blueprints/Units/PlayerUnit.PlayerUnit_C|GetControlRadius _output_get))
  (Transformation|AttachActorToActor (Variables|Default|GetPlayer) "None" "SnapToTarget" "SnapToTarget" "SnapToTarget" false)
  (for _index (range 0 (Variables|Default|GetGridSize))
    (for _index_2 (range 0 (Variables|Default|GetGridSize))
      (bind _returnvalue_2 (Game|SpawnActorfromClass "/Game/Golem/Blueprints/Units/GridCell.GridCell_C" (Math|Transform|MakeTransform (Math|Vector|MakeVector (* (- _index_2 _returnvalue) (Variables|Default|GetGridCellSize)) (* (- _index _returnvalue) (Variables|Default|GetGridCellSize)) 0.0) "0, 0, 0" (Math|Vector|MakeVector 0.5 0.5 0.1)) "AlwaysSpawn" 0 0))
      (Transformation|AttachActorToActor _returnvalue_2 self "None" "KeepRelative" "KeepRelative" "KeepWorld" true)
      (Utilities|Array|Add (Variables|Default|GetCells) 0)))
  (Rendering|SetVisibility (Variables|Default|GetDefaultSceneRoot) false true))

(event Collision|EventActorBeginOverlap
  (params (OtherActor :type Actor%20Object%20Reference)))

(event EventTick
  (params (DeltaSeconds :type Float%20%28single-precision%29)))

(fn ConstructionScript)