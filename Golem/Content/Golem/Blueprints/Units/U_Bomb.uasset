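; Bomb unit for the player that explodes near its anchor when outside control range, or on death, once its cooldown allows.
; Explosions damage and knock back enemy-tagged pawns through GolemInterface, then the body scales back up as it recharges.
; Merging keeps the best stat multipliers, destroys the other units and offers a two-tier skill choice via the player's BombWidget.
; Skills alter cooldown, radius, knockback or lava spawning; Leftover Scraps and Singularity only set flags here.
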(event Custom|Bomb%20Merge
  (bind _asplayer_unit (Utilities|Casting|CastToPlayerUnit (Game|Player|GetPlayerPawn 0)))
  (Variables|Default|SetAs%20Player%20Unit _asplayer_unit)
  (Variables|Default|SetButtonholder (Variables|/Game/Golem/UI/MergeMenues/BombMergeMenu.BombMergeMenu_C|GetButtonholder (Variables|/Game/Golem/Blueprints/Units/PlayerUnit.PlayerUnit_C|GetBomb%20Widget _asplayer_unit)))
  (if (== self (Variables|/Game/Golem/Blueprints/Units/PlayerUnit.PlayerUnit_C|GetMainMergeUnit (Variables|Default|GetAs%20Player%20Unit)))
    ;[1 1 1] Stat setting
    (for _array_element (Variables|/Game/Golem/Blueprints/Units/PlayerUnit.PlayerUnit_C|GetMergeUnits (Variables|Default|GetAs%20Player%20Unit))
      (if (> (Variables|/Game/Golem/Blueprints/Units/Unit.Unit_C|GetAttackDamageMultiplier _array_element) (Variables|Default|GetAttackDamageMultiplier))
        (Variables|Default|SetAttackDamageMultiplier (Variables|/Game/Golem/Blueprints/Units/Unit.Unit_C|GetAttackDamageMultiplier _array_element))))
    (for _array_element_2 (Variables|/Game/Golem/Blueprints/Units/PlayerUnit.PlayerUnit_C|GetMergeUnits (Variables|Default|GetAs%20Player%20Unit))
      (if (not (> (Variables|/Game/Golem/Blueprints/Units/Unit.Unit_C|GetAttackCoolDownMultiplier _array_element_2) (Variables|Default|GetAttackCoolDownMultiplier)))
        (Variables|Default|SetAttackCoolDownMultiplier (Variables|/Game/Golem/Blueprints/Units/Unit.Unit_C|GetAttackCoolDownMultiplier _array_element_2))))
    (for _array_element_3 (Variables|/Game/Golem/Blueprints/Units/PlayerUnit.PlayerUnit_C|GetMergeUnits (Variables|Default|GetAs%20Player%20Unit))
      (if (> (Variables|/Game/Golem/Blueprints/Units/Unit.Unit_C|GetDefenceMultiplier _array_element_3) (Variables|Default|GetDefenceMultiplier))
        (Variables|Default|SetDefenceMultiplier (Variables|/Game/Golem/Blueprints/Units/Unit.Unit_C|GetDefenceMultiplier _array_element_3))))
    (for _array_element_4 (Variables|/Game/Golem/Blueprints/Units/PlayerUnit.PlayerUnit_C|GetMergeUnits (Variables|Default|GetAs%20Player%20Unit))
      (if (> (Variables|/Game/Golem/Blueprints/Units/Unit.Unit_C|GetMaxHealthMultiplier _array_element_4) (Variables|Default|GetMaxHealthMultiplier))
        (Variables|Default|SetMaxHealthMultiplier (Variables|/Game/Golem/Blueprints/Units/Unit.Unit_C|GetMaxHealthMultiplier _array_element_4))))
    (bind _array_element_5 (Utilities|Array|ForEachLoopwithBreak (Variables|/Game/Golem/Blueprints/Units/PlayerUnit.PlayerUnit_C|GetMergeUnits (Variables|Default|GetAs%20Player%20Unit)))
      (:LoopBody
        (if (not (== _array_element_5 (Variables|/Game/Golem/Blueprints/Units/PlayerUnit.PlayerUnit_C|GetMainMergeUnit (Variables|Default|GetAs%20Player%20Unit))))
          (Actor|DestroyActor _array_element_5)))
      (:Completed
        ;[1 1 1] Adding skills (ints) to array
        (Utilities|Array|Clear (Variables|Default|GetAwailable%20skills))
        (for _index (range 0 5)
          (switch int _index
            (:0
              ;[1 1 1] Quick assembly
              (if (not (Variables|Default|GetHasQuickAssembly))
                (Utilities|Array|Add (Variables|Default|GetAwailable%20skills) (+ 0 0))))
            (:1
              ;[1 1 1] plothole
              (if (not (Variables|Default|GetHasPlothole))
                (Utilities|Array|Add (Variables|Default|GetAwailable%20skills) (+ 0 1))))
            (:2
              ;[1 1 1] Impact
              (if (not (Variables|Default|GetHasImpact))
                (Utilities|Array|Add (Variables|Default|GetAwailable%20skills) (+ 0 2))))
            (:3
              ;[1 1 1] LOS
              (if (Variables|Default|GetHasQuickAssembly)
                (if (not (Variables|Default|GetHasLeftOverScraps))
                  (Utilities|Array|Add (Variables|Default|GetAwailable%20skills) (+ 0 3)))))
            (:4
              ;[1 1 1] Oozing Liquid
              (if (Variables|Default|GetHasPlothole)
                (if (not (Variables|Default|GetHasOozingLiquid))
                  (Utilities|Array|Add (Variables|Default|GetAwailable%20skills) (+ 0 4)))))
            (:5
              ;[1 1 1] Singularity
              (if (Variables|Default|GetHasImpact)
                (if (not (Variables|Default|GetHasSingularity))
                  (Utilities|Array|Add (Variables|Default|GetAwailable%20skills) (+ 0 5)))))))
        ;[1 1 1] Creating buttons
        (for (_array_element_6 _array_index) (Variables|Default|GetAwailable%20skills)
          (for (_array_element_7 _array_index_2) (Class|PanelWidget|GetAllChildren (Variables|Default|GetButtonholder))
            (if (or (== (* _array_index 2) _array_index_2) (== (+ (* _array_index 2) 1) _array_index_2))
              (bind _astext (Utilities|Casting|CastToTextBlock _array_element_7)
                (:then
                  (Widget|SetVisibility _array_element_7 "Visible")
                  ;[1 1 1] Setting Text description
                  (switch int _array_element_6
                    (:0
                      (Rendering|Components|TextRender|SetText _astext "Quick Assembly"))
                    (:1
                      (Rendering|Components|TextRender|SetText _astext "Plothole"))
                    (:2
                      (Rendering|Components|TextRender|SetText _astext "Impact"))
                    (:3
                      (Rendering|Components|TextRender|SetText _astext "Leftover Scraps"))
                    (:4
                      (Rendering|Components|TextRender|SetText _astext "Oozing Liquid"))
                    (:5
                      (Rendering|Components|TextRender|SetText _astext "Singularity"))))
                (:CastFailed
                  (Widget|SetVisibility _array_element_7 "Visible"))))))))))

(event Custom|BombUpgrade
  (bind _as_player_unit (Variables|Default|GetAs%20Player%20Unit))
  (bind _mainmergeunit (Variables|/Game/Golem/Blueprints/Units/PlayerUnit.PlayerUnit_C|GetMainMergeUnit _as_player_unit))
  ;[1 1 1] Checking Array and setting Corresponding Boolean (skill) to true
  (bind (_array_element _array_index) (Utilities|Array|ForEachLoopwithBreak (Variables|Default|GetAwailable%20skills) :!label _label)
    (:LoopBody
      (if (== _array_index (Variables|Default|GetASpos))
        (switch int _array_element
          (:0
            (CallFunction|QuickAssembly))
          (:1
            (CallFunction|Plothole))
          (:2
            (CallFunction|Impact))
          (:3
            (CallFunction|LeftoverScraps))
          (:4
            (CallFunction|OozingLiquid))
          (:5
            (CallFunction|Singularity)))
        (Variables|Default|SetASpos 0)
        (Variables|/Game/Golem/Blueprints/Units/Unit.Unit_C|SetMerges _mainmergeunit (+ (Variables|/Game/Golem/Blueprints/Units/Unit.Unit_C|GetMerges _mainmergeunit) 1))
        (Utilities|Array|Clear (Variables|/Game/Golem/Blueprints/Units/PlayerUnit.PlayerUnit_C|GetMergeUnits _as_player_unit))
        (for _array_element_2 (Class|PanelWidget|GetAllChildren (Variables|Default|GetButtonholder))
          (Widget|SetVisibility _array_element_2 "Collapsed"))
        (Widget|RemovefromParent (Variables|/Game/Golem/Blueprints/Units/PlayerUnit.PlayerUnit_C|GetBomb%20Widget _as_player_unit))
        (goto _label Break)))))

(event EventBeginPlay
  (Variables|/Script/Engine.CharacterMovementComponent|SetMaxWalkSpeed (Variables|Character|GetCharacterMovement) (Variables|Default|GetMovementSpeed))
  (Transformation|AttachActorToActor (Game|Player|GetPlayerPawn 0) "None" "KeepWorld" "KeepWorld" "KeepWorld" true)
  (Variables|Default|SetTimeSinceLastAttack (Variables|Default|GetAttackCoolDown))
  (Variables|Default|SetAnchor (- (Transformation|GetActorLocation self) (Transformation|GetActorLocation (Game|Player|GetPlayerPawn 0))))
  (Utilities|Array|Add (Variables|Default|GetShells) (Variables|Default|Getshell1))
  (Utilities|Array|Add (Variables|Default|GetShells) (Variables|Default|Getshell2))
  (Utilities|Array|Add (Variables|Default|GetShells) (Variables|Default|Getshell3))
  (Utilities|Array|Add (Variables|Default|GetShells) (Variables|Default|Getshell4))
  (Utilities|Array|Add (Variables|Default|GetShells) (Variables|Default|Getshell5))
  (Utilities|Array|Add (Variables|Default|GetShells) (Variables|Default|Getshell6))
  (Utilities|Array|Add (Variables|Default|GetShells) (Variables|Default|Getshell7))
  (Utilities|Array|Add (Variables|Default|GetShells) (Variables|Default|Getshell8)))

(event EventTick
  (params (DeltaSeconds :type Float%20%28single-precision%29))
  (bind _returnvalue (Transformation|GetActorLocation))
  (bind _anchor (Variables|Default|GetAnchor))
  (bind _attackcooldown (Variables|Default|GetAttackCoolDown))
  (bind _timesincelastattack (Variables|Default|GetTimeSinceLastAttack))
  (bind _attackcooldownmultiplier (Variables|Default|GetAttackCoolDownMultiplier))
  (bind _returnvalue_2 (* _attackcooldown _attackcooldownmultiplier))
  (bind _returnvalue_3 (> _timesincelastattack _returnvalue_2))
  (|CallParentFunction DeltaSeconds)
  (Utilities|FlowControl|Sequence
    (:then_0
      (if (not (Variables|Default|GetInControlRange))
        (if (< (Math|Vector|Distance2D(Vector) (Math|Vector2D|MakeVector2D (.x _returnvalue) (.y _returnvalue)) (Math|Vector2D|MakeVector2D (.x _anchor) (.y _anchor))) 1e+02)
          (if _returnvalue_3
            (if (not (Variables|Default|GetHasExploded))
              (CallFunction|Explode))))))
    (:then_1
      (if (not _returnvalue_3)
        (Transformation|SetRelativeScale3D (Variables|Default|GetBody) (* "1.000000,1.000000,1.000000" (/ _timesincelastattack _returnvalue_2)))))))

(event EventAttack
  (if (> (Variables|Default|GetHealth) 0.0)
    (if (> (Variables|Default|GetTimeSinceLastAttack) (* (Variables|Default|GetAttackCoolDown) (Variables|Default|GetAttackCoolDownMultiplier)))
      _)))

(fn ConstructionScript
  (|CallParentFunction)
  (Rendering|Material|SetMaterial (Variables|Default|Getcrystal) 0 (Variables|Default|GetCrystalMaterial)))

(fn Explode
  (Variables|Default|SetHasExploded true)
  (Components|Activation|Activate (Variables|Default|GetExplosion) true)
  (Variables|Default|SetTimeSinceLastAttack 0.0)
  (Transformation|SetRelativeScale3D (Variables|Default|GetBody) "0, 0, 0")
  (if (or (Variables|Default|GetHasPlothole) (Variables|Default|GetHasOozingLiquid))
    (Game|SpawnActorfromClass "/Game/Golem/Blueprints/LavaGround.LavaGround_C" (Transformation|GetWorldTransform (Variables|Default|GetLavaGround)) "Undefined" 0 0))
  (bind _outactors (Collision|SphereOverlapActors (Transformation|GetActorLocation) (Variables|Default|GetExplosionRadius) (Utilities|Array|MakeArray "ObjectTypeQuery3") 0))
  (for _array_element _outactors
    (if (and (Utilities|DoesObjectImplementInterface _array_element "/Game/Golem/Blueprints/GolemInterface.GolemInterface_C") (Actor|ActorHasTag _array_element "Enemy"))
      (bind _asgolem_interface (Utilities|Casting|CastToGolemInterface _array_element))
      (bind _knockbackvector (CallFunction|GetKnockback _array_element))
      (Default|Attacked _asgolem_interface (* (Variables|Default|GetAttackDamage) (Variables|Default|GetAttackDamageMultiplier)) _knockbackvector))))

(fn OnSelected
  (if (Variables|Default|GetIsSelected)
    (Variables|Default|SetIsSelected false)
    (Rendering|SetVisibility (Variables|Default|GetSelectCircle) false false)
    (Variables|Default|SetHasExploded false)
    (else
      (Variables|Default|SetIsSelected true)
      (Rendering|SetVisibility (Variables|Default|GetSelectCircle) true false))))

(fn QuickAssembly
  (Variables|Default|SetHasQuickAssembly true)
  (Variables|Default|SetAttackCoolDown 6e+01)
  (Variables|Default|SetAttackDamage (- (Variables|Default|GetAttackDamage) 15.0))
  (Variables|Default|SetExplosionRadius (* (Variables|Default|GetExplosionRadius) 0.3)))

(fn Death
  (if (> (Variables|Default|GetTimeSinceLastAttack) (Variables|Default|GetAttackCoolDown))
    (CallFunction|Explode)))

(fn Plothole
  (Variables|Default|SetHasPlothole true))

(fn Impact
  (Variables|Default|SetHasImpact true)
  (Variables|Default|SetKnockback (* 3 (Variables|Default|GetKnockback))))

(fn LeftoverScraps
  (Variables|Default|SetHasLeftOverScraps true))

(fn OozingLiquid
  (Variables|Default|SetHasOozingLiquid true)
  (Transformation|SetRelativeScale3D (Variables|Default|GetLavaGround) (* (Variables|/Script/Engine.SceneComponent|GetRelativeScale3D (Variables|Default|GetLavaGround)) 2.0)))

(fn Singularity
  (Variables|Default|SetHasSingularity true))