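; EnemyUnit is an apparent base enemy unit with health, cooldown-gated attacks, block, defence, knockback and repair, leaving TickFunction and LevelUp empty.
; Timelines animate its meshes for rising, hovering, damage shake, death and sinking, while a dynamic crystal material glows with health.
; Attacked applies knockback and unblocked damage.
; At zero health it unpossesses, topples, then randomly spawns a temporary Corpse or Scrap before sinking and being destroyed.
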(event Custom|Sink
  (bind _location (Timeline|SinkAnim Play)
    (:Update
      (Transformation|SetRelativeLocation (Variables|Default|GetMeshes) (Math|Vector|MakeVector 0.0 0.0 (* _location (* (Variables|/Script/Engine.CapsuleComponent|GetCapsuleRadius (Variables|Collision|GetCapsuleComponent)) 1.5))) false false))
    (:Finished
      (Actor|DestroyActor))))

(event Custom|StartAnim
  (bind _hover (Variables|Default|GetHover))
  (bind _location (Timeline|RiseAnim PlayFromStart)
    (:Update
      (Transformation|SetRelativeLocation (Variables|Default|GetMeshes) (Math|Vector|MakeVector 0.0 0.0 (* _location (* (Variables|/Script/Engine.CapsuleComponent|GetCapsuleRadius (Variables|Collision|GetCapsuleComponent)) 1.5))) false false)
      (if (< _location -1.0)
        (Components|Activation|Activate (Variables|Default|GetP_DeathDust) true)))
    (:Finished
      (Audio|Components|Audio|Play _hover)
      (Components|Timeline|SetPlaybackPosition _hover (* (Math|Random|RandomFloat) (Components|Timeline|GetTimelineLength _hover)) false true))))

(event EventBeginPlay
  (CallFunction|Init))

(event EventRepair
  (params (Amount :type Float%20%28single-precision%29))
  (Variables|Default|SetHealth (Math|Float|Clamp(Float) (+ (Variables|Default|GetHealth) Amount) 0.0 (* (Variables|Default|GetMaxHealth) (Variables|Default|GetMaxHealthMultiplier))))
  (Components|Activation|Activate (Variables|Components|GetRepairEffect) true)
  (CallFunction|UpdateShowHealth))

(event EventAttack
  (if (> (Variables|Default|GetHealth) 0.0)
    (if (> (Variables|Default|GetTimeSinceLastAttack) (Variables|Default|GetAttackCoolDown))
      (Variables|Default|SetTimeSinceLastAttack 0.0))))

(event EventTick
  (params (DeltaSeconds :type Float%20%28single-precision%29))
  (if (>= (Variables|Default|GetHealth) 0.0)
    (Variables|Default|SetTimeSinceLastAttack (+ DeltaSeconds (Variables|Default|GetTimeSinceLastAttack)))
    (Utilities|FlowControl|Sequence
      (:then_0
        (CallFunction|TickFunction)))))

(event EventMoveUnit
  (params (TargetLocation :type Vector :default "0, 0, 0"))
  (Class|GolemInterface|MoveUnit(Message) (Pawn|GetController) TargetLocation))

(event EventAttacked
  (params (AttackDamage :type Float%20%28single-precision%29) (AttackKnockback :type Vector :default "0, 0, 0"))
  (bind _feet (Variables|Components|GetFeet))
  (if (> (Variables|Default|GetHealth) 0.0)
    (Transformation|AddActorWorldOffset AttackKnockback)
    (if (>= (Variables|Default|GetHealth) 0.0)
      (bind _isblocked (CallFunction|BlockAttack))
      (if (not _isblocked)
        (bind _returnvalue (CallFunction|TakeDamage AttackDamage))
        (Audio|Components|Audio|Stop (Variables|Default|GetHover))
        (bind _shake (Timeline|DamageShake PlayFromStart)
          (:Update
            (Transformation|SetRelativeLocation (Variables|Default|GetMeshes) (Math|Vector|MakeVector 0.0 0.0 (* (* _shake 1e+02) (/ (+ _returnvalue 1.0) 2.0))) false false))
          (:Finished
            (Components|Timeline|PlayfromStart (Variables|Default|GetHover))
            (if (<= (Variables|Default|GetHealth) 0.0)
              ;[1 1 1] Death
              (Transformation|DetachFromActor "KeepWorld" "KeepWorld" "KeepWorld")
              (Audio|Components|Audio|Stop (Variables|Default|GetHover))
              (Variables|/Script/Engine.PrimitiveComponent|SetbGenerateOverlapEvents (Variables|Collision|GetCapsuleComponent) false)
              (Pawn|UnPossess (Pawn|GetController))
              (Components|Activation|Activate (Variables|Default|GetDeathExplosion) true)
              (Transformation|SetRelativeLocation _feet (Math|Vector|MakeVector 0.0 0.0 (* (Variables|/Script/Engine.CapsuleComponent|GetCapsuleHalfHeight (Variables|Collision|GetCapsuleComponent)) -1.0)) false false)
              (bind (_direction _rotation _spin) (Timeline|DeathAnim PlayFromStart)
                (:Update
                  (Transformation|SetRelativeRotation _feet (Math|Rotator|MakeRotator 0.0 (* _rotation 9e+01) (* _spin 1.2e+02)) false false))
                (:Finished
                  (Components|Activation|Activate (Variables|Default|GetP_DeathDust) true)
                  (if (< (Math|Random|RandomFloat) (Variables|Default|GetChanceSpawnCorpse))
                    (bind _returnvalue_2 (Game|SpawnActorfromClass (Variables|Default|GetCorpse) (Transformation|GetActorTransform) "AlwaysSpawn" 0 0))
                    (bind _ascorpse (Utilities|Casting|CastToCorpse _returnvalue_2))
                    (Variables|/Game/Golem/Blueprints/Corpses/Corpse.Corpse_C|SetSpawnedFrom _ascorpse self)
                    (Utilities|FlowControl|Delay 3e+01)
                    (Actor|DestroyActor _returnvalue_2)
                    (CallFunction|Sink)
                    (else
                      (CallFunction|SpawnScrap)
                      (CallFunction|Sink))))))))))))

(fn ConstructionScript
  (bind _returnvalue (Transformation|GetActorLocation))
  (Variables|Default|SetHealth (Variables|Default|GetMaxHealth))
  (bind _returnvalue_2 (Rendering|Material|CreateDynamicMaterialInstance "/Game/Golem/GolemMaterials/M_crystal.M_crystal" "None" "None" :!class /Script/Engine.KismetMaterialLibrary))
  (Variables|Default|SetCrystalMaterial _returnvalue_2)
  (Class|TimelineComponent|SetFloatCurve (Variables|Default|GetDamageShake) "/Game/Golem/Blueprints/Shake.Shake" "Shake")
  (Class|TimelineComponent|SetFloatCurve (Variables|Default|GetDeathAnim) "/Game/Golem/Blueprints/DeathCurve.DeathCurve" "Rotation")
  (Transformation|SetActorLocation (Math|Vector|MakeVector (.x _returnvalue) (.y _returnvalue) (Variables|/Script/Engine.CapsuleComponent|GetCapsuleHalfHeight (Variables|Collision|GetCapsuleComponent))) false false))

(fn AngleRange
  (params (AngleIn :type Float%20%28single-precision%29))
  (LocalVariables|SetAngle AngleIn)
  (while (< (LocalVariables|GetAngle) 0.0)
    (LocalVariables|SetAngle (+ (LocalVariables|GetAngle) 3.6e+02)))
  (while (< 3.6e+02 (LocalVariables|GetAngle))
    (LocalVariables|SetAngle (- (LocalVariables|GetAngle) 3.6e+02)))
  (return (LocalVariables|GetAngle)))

(fn BlockAttack
  (return (< (Math|Random|RandomFloat) (Variables|Default|GetBlock))))

(fn TakeDamage
  (params (damage :type Float%20%28single-precision%29))
  (bind _defencemultiplier (Variables|Default|GetDefenceMultiplier))
  (bind _defence (Variables|Default|GetDefence))
  (bind _returnvalue (* _defence _defencemultiplier))
  (bind _returnvalue_2 (- 1.0 _returnvalue))
  (bind _returnvalue_3 (* damage _returnvalue_2))
  (Variables|Default|SetHealth (- (Variables|Default|GetHealth) _returnvalue_3))
  (CallFunction|UpdateShowHealth)
  (return (/ _returnvalue_3 (Variables|Default|GetMaxHealth))))

(fn GetDeltaMove
  (params (deltaSeconds :type Float%20%28single-precision%29))
  (bind _returnvalue (Transformation|GetActorLocation))
  (bind _output_get (Variables|Default|SetDeltaMove (* (* (- _returnvalue (Variables|Default|GetPreviousLocation)) deltaSeconds) 1e+02)))
  (Variables|Default|SetPreviousLocation _returnvalue))

(fn GetKnockback
  (params (Target :type Actor%20Object%20Reference))
  (bind _returnvalue (Transformation|GetActorLocation Target))
  (bind _returnvalue_2 (Transformation|GetActorLocation))
  (bind _returnvalue_3 (- _returnvalue _returnvalue_2))
  (return (* (Math|Vector|Normalize (Math|Vector|MakeVector (.x _returnvalue_3) (.y _returnvalue_3) 0.0)) (Variables|Default|GetKnockback))))

(fn Init
  (Variables|Default|SetTimeSinceLastAttack (Variables|Default|GetAttackCoolDown))
  (Variables|/Script/Engine.CharacterMovementComponent|SetMaxWalkSpeed (Variables|Character|GetCharacterMovement) (Variables|Default|GetMovementSpeed))
  (CallFunction|StartAnim))

(fn UpdateShowHealth
  (Rendering|Material|SetScalarParameterValue (Variables|Default|GetCrystalMaterial) "Glow" (/ (Variables|Default|GetHealth) (Variables|Default|GetMaxHealth)) :!class /Script/Engine.MaterialInstanceDynamic))

(fn SpawnScrap
  (Game|SpawnActorfromClass "/Game/Golem/Blueprints/Enemies/Scrap.Scrap_C" (Transformation|GetActorTransform) "AlwaysSpawn" 0 0))

(fn LevelUp)

(fn TickFunction)