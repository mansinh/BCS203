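; Enemy AI controller that runs the enemy behavior tree and feeds it player detection data.
; Each tick it sphere-overlaps pawns within the controlled Enemy's DetectRange and picks the nearest one tagged Player by squared distance.
; It writes TargetDetected and TargetLocation to the Blackboard, then sets the Enemy's TargetActor and the controller's focal point to that player.
; A MoveUnit event offers simple move-to-location.
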(event EventBeginPlay
  (AI|RunBehaviorTree "/Game/Golem/Blueprints/Enemies/EnemyBehaviourTree.EnemyBehaviourTree"))

(event EventMoveUnit
  (params (TargetLocation :type Vector :default "0, 0, 0"))
  (AI|Navigation|SimpleMovetoLocation self TargetLocation))

(event EventTick
  (params (DeltaSeconds :type Float%20%28single-precision%29))
  (bind _blackboard (Variables|Default|GetBlackboard))
  (bind _asenemy (Utilities|Casting|CastToEnemy (Pawn|GetControlledPawn)))
  (bind _outactors (Collision|SphereOverlapActors (Transformation|GetActorLocation _asenemy) (Variables|/Game/Golem/Blueprints/Enemies/Enemy.Enemy_C|GetDetectRange _asenemy) (Utilities|Array|MakeArray "ObjectTypeQuery3") 0 (Utilities|Array|MakeArray _asenemy)))
  (bind _targetactor (CallFunction|FindClosestActor _outactors (Transformation|GetActorLocation _asenemy) (Variables|/Game/Golem/Blueprints/Enemies/Enemy.Enemy_C|GetDetectRange _asenemy) "Player"))
  (AI|Components|Blackboard|SetValueasBool _blackboard (Utilities|Name|MakeLiteralName "TargetDetected") (Utilities|IsValid _targetactor))
  (if (Utilities|IsValid _targetactor)
    (AI|Components|Blackboard|SetValueasVector _blackboard (Utilities|Name|MakeLiteralName "TargetLocation") (Transformation|GetActorLocation _targetactor))
    (bind _output_get (Variables|/Game/Golem/Blueprints/Enemies/Enemy.Enemy_C|SetTargetActor _asenemy _targetactor))
    (AI|SetFocalPoint (Transformation|GetActorLocation _output_get))
    (Utilities|FlowControl|Delay 1.0)))

(fn ConstructionScript)

(fn FindClosestActor
  (params (Actors :type Array%20of%20Actor%20Object%20References) (Position :type Vector) (Range :type Float%20%28single-precision%29) (Tag :type Name))
  (LocalVariables|SetClosestSqDist (* Range Range))
  (LocalVariables|SetClosestActor 0)
  (for _array_element Actors
    (if (Actor|ActorHasTag _array_element Tag)
      (if (< (Class|KismetMathLibrary|VectorDistanceSquared (Transformation|GetActorLocation _array_element) Position) (LocalVariables|GetClosestSqDist))
        (LocalVariables|SetClosestSqDist (Class|KismetMathLibrary|VectorDistanceSquared (Transformation|GetActorLocation _array_element) Position))
        (LocalVariables|SetClosestActor _array_element))))
  (return (LocalVariables|GetClosestActor)))