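; Enemy melee character that spawns its default controller and forwards move orders to it.
; Attack is gated by a Tick-accumulated cooldown, faces TargetActor, then sphere-traces from the target to the melee point.
; Hits play an impact effect and damage a PlayerUnit directly or other actors through GolemInterface.
; Incoming hits apply knockback and reduce health; death triggers an explosion, hides the mesh, spawns a corpse and destroys the actor after a delay.
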(event EventBeginPlay
  (Variables|/Script/Engine.CharacterMovementComponent|SetMaxWalkSpeed (Variables|Character|GetCharacterMovement) (Variables|Default|GetMaxMoveSpeed))
  (Pawn|SpawnDefaultController))

(event EventTick
  (params (DeltaSeconds :type Float%20%28single-precision%29))
  (if (>= (Variables|Default|GetHealth) 0.0)
    (Variables|Default|SetTimeSinceLastAttack (+ DeltaSeconds (Variables|Default|GetTimeSinceLastAttack)))))

(event EventAttack
  (if (> (Variables|Default|GetTimeSinceLastAttack) (Variables|Default|GetAttackCoolDown))
    (CallFunction|AttackTarget)
    (Variables|Default|SetTimeSinceLastAttack 0.0)))

(event EventMoveUnit
  (params (TargetLocation :type Vector :default "0, 0, 0"))
  (Class|GolemInterface|MoveUnit(Message) (Pawn|GetController) TargetLocation))

(event EventAttacked
  (params (AttackDamage :type Float%20%28single-precision%29) (AttackKnockback :type Vector :default "0, 0, 0"))
  (Transformation|AddActorWorldOffset AttackKnockback)
  (if (>= (Variables|Default|GetHealth) 0.0)
    (Variables|Default|SetHealth (- (Variables|Default|GetHealth) AttackDamage))
    (if (< (Variables|Default|GetHealth) 0.0)
      (Components|Activation|Activate (Variables|Default|GetDeathExplosion) true)
      (Rendering|SetVisibility (Variables|Default|GetPlaceholderMesh) false false)
      (Game|SpawnActorfromClass (Variables|Default|GetCorpse) (Transformation|GetActorTransform) "Undefined" 0 0)
      (Utilities|FlowControl|Delay 0.5)
      (Actor|DestroyActor))))

(fn ConstructionScript
  (Variables|Default|SetHealth (Variables|Default|GetMaxHealth)))

(fn AttackTarget
  (bind _meleeattackimpact (Variables|Default|GetMeleeAttackImpact))
  (bind _meleeattackimpact_2 (Variables|Default|GetMeleeAttackImpact))
  (bind _targetactor (Variables|Default|GetTargetActor))
  (Transformation|SetWorldRotation (Variables|Collision|GetCapsuleComponent) (Math|Rotator|FindLookatRotation (Transformation|GetActorLocation) (Transformation|GetActorLocation _targetactor)) false false)
  (bind _outhit (Collision|SphereTraceByChannel (Transformation|GetActorLocation _targetactor) (Transformation|GetWorldLocation (Variables|Default|GetMeleeAttackPosition)) 2e+01 "TraceTypeQuery2" false 0 "None"))
  (bind _asplayer_unit (Utilities|Casting|CastToPlayerUnit (.HitActor (Collision|BreakHitResult _outhit)))
    (:then
      (Transformation|SetWorldLocation _meleeattackimpact_2 (.ImpactPoint (Collision|BreakHitResult _outhit)) false false)
      (Components|Activation|Activate _meleeattackimpact_2 false)
      (Default|Attacked _asplayer_unit (Variables|Default|GetAttackDamage) "0, 0, 0"))
    (:CastFailed
      (if (Utilities|DoesObjectImplementInterface (.HitActor (Collision|BreakHitResult _outhit)) "/Game/Golem/Blueprints/GolemInterface.GolemInterface_C")
        (Transformation|SetWorldLocation _meleeattackimpact (.ImpactPoint (Collision|BreakHitResult _outhit)) false false)
        (Components|Activation|Activate _meleeattackimpact false)
        (Class|GolemInterface|Attacked(Message) (.HitActor (Collision|BreakHitResult _outhit)) (Variables|Default|GetAttackDamage) "0, 0, 0")))))