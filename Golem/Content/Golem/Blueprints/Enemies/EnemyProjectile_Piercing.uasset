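; Piercing enemy projectile that damages players it passes through and survives until its hit count runs out.
; On ending an overlap, it decrements Hits, sends player-tagged GolemInterface actors a no-knockback attack message and activates its Hit component.
; When Hits runs out on a player, it hides the mesh and destroys itself after a delay; any other valid actor destroys it immediately.
; The construction script sets movement speed from Speed.
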(event Collision|EventActorEndOverlap
  (params (OtherActor :type Actor%20Object%20Reference))
  (Utilities|IsValid OtherActor
    (:Is%20Valid
      (Math|Integer|DecrementInt (Variables|Default|GetHits)
        (:%20%20
          (if (and (Utilities|DoesObjectImplementInterface OtherActor "/Game/Golem/Blueprints/GolemInterface.GolemInterface_C") (Actor|ActorHasTag OtherActor "Player"))
            (Class|GolemInterface|Attacked(Message) OtherActor (Variables|Default|GetAttackDamage) "0, 0, 0")
            (Components|Activation|Activate (Variables|Default|GetHit) true)
            (if (<= (Variables|Default|GetHits) 0)
              (Rendering|SetVisibility (Variables|Default|GetProjectileMesh) false false)
              (Utilities|FlowControl|Delay 2.0)
              (Actor|DestroyActor :!label _label))
            (else
              (goto _label))))))))

(fn ConstructionScript
  (Variables|/Script/Engine.ProjectileMovementComponent|SetInitialSpeed (Variables|Default|GetProjectileMovement) (Variables|Default|GetSpeed)))