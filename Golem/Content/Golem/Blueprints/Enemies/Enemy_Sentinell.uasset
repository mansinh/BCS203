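; Sentinel enemy character that fires projectiles at a target actor it can see.
; BeginPlay applies its maximum walk speed and spawns its default controller.
; ShootTarget checks line of sight to slightly above the target's origin, aims the muzzle component, activates particles and spawns a projectile; its fire sound is disconnected.
; The Attack event only tests the cooldown and does not call ShootTarget.
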(event EventBeginPlay
  (Variables|/Script/Engine.CharacterMovementComponent|SetMaxWalkSpeed (Variables|Character|GetCharacterMovement) (Variables|Default|GetMaxMoveSpeed))
  (Pawn|SpawnDefaultController))

(event Collision|EventActorBeginOverlap
  (params (OtherActor :type Actor%20Object%20Reference)))

(event EventTick
  (params (DeltaSeconds :type Float%20%28single-precision%29))
  (|CallParentFunction DeltaSeconds) ; This node is disabled and will not be called.\nDrag off pins to build functionality.
)

(event EventAttack
  (if (> (Variables|Default|GetTimeSinceLastAttack) (Variables|Default|GetAttackCoolDown))
    _))

(fn ConstructionScript
  (|CallParentFunction))

(fn ShootTarget
  (bind _targetactor (Variables|Default|GetTargetActor))
  (bind _shootfromposition (Variables|Default|GetShootFromPosition))
  (bind _returnvalue (Transformation|GetActorLocation _targetactor))
  (bind _returnvalue_2 (Transformation|GetWorldLocation _shootfromposition))
  (bind _returnvalue_3 (+ _returnvalue (Math|Vector|MakeVector 0.0 0.0 15.0)))
  (bind _result (CallFunction|HasLineOfSight _returnvalue_2 _returnvalue_3 (Utilities|Array|MakeArray self _targetactor)))
  (if _result
    (Transformation|SetWorldRotation _shootfromposition (Math|Rotator|FindLookatRotation _returnvalue_2 _returnvalue_3) false false)
    (Components|Activation|Activate (Variables|Default|GetParticleSystem) true)
    (Game|SpawnActorfromClass "/Game/Golem/Blueprints/Enemies/EnemyProjectile.EnemyProjectile_C" (Transformation|GetWorldTransform (Variables|Default|GetShootFromPosition)) "AlwaysSpawn" 0 (Variables|Default|GetProjectileSpeed) 0)))