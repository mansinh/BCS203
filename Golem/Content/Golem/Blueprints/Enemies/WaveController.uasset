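; WaveController is an enemy spawner that escalates pressure around the player.
; A delayed BeginPlay loop spawns while "Enemy"-tagged actors are below MaxEnemyCount, picking basic, Shooter or Sentinell through cascading probability rolls that may spawn none.
; Spawn points offset the player's location by SpawnRadius-scaled sine and cosine of independent random angles, so they are not confined to a circle.
; Each Tick raises the capped enemy limit and shrinks SpawnTime geometrically.
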(event EventBeginPlay
  (if (< (Utilities|Array|Length (stale _outactors)) (Math|Float|Truncate (Variables|Default|GetMaxEnemyCount))) :!label _label
    (bind _returnvalue (CallFunction|RandomTransform))
    (if (< (Math|Random|RandomFloat) (Utilities|Array|Get(acopy) (Variables|Default|GetSpawnProbabilities)))
      (Game|SpawnActorfromClass "/Game/Golem/Blueprints/Enemies/Enemy.Enemy_C" _returnvalue "AdjustIfPossibleButAlwaysSpawn" 0 0 3e+03 0)
      (elif (< (Math|Random|RandomFloat) (Utilities|Array|Get(acopy) (Variables|Default|GetSpawnProbabilities) 1))
        (Game|SpawnActorfromClass "/Game/Golem/Blueprints/Enemies/Enemy_Shooter.Enemy_Shooter_C" _returnvalue "AdjustIfPossibleButAlwaysSpawn" 0 0 3e+03 0)
        (elif (< (Math|Random|RandomFloat) (Utilities|Array|Get(acopy) (Variables|Default|GetSpawnProbabilities) 2))
          (Game|SpawnActorfromClass "/Game/Golem/Blueprints/Enemies/Enemy_Sentinell.Enemy_Sentinell_C" _returnvalue "AdjustIfPossibleButAlwaysSpawn" 0 0 3e+03 0)))))
  (Utilities|FlowControl|Delay (Variables|Default|GetSpawnTime))
  (bind _outactors (Actor|GetAllActorswithTag "Enemy"))
  (goto _label))

(event Collision|EventActorBeginOverlap
  (params (OtherActor :type Actor%20Object%20Reference)))

(event EventTick
  (params (DeltaSeconds :type Float%20%28single-precision%29))
  (Variables|Default|SetMaxEnemyCount (Math|Float|Clamp(Float) (+ (Variables|Default|GetMaxEnemyCount) 1.0) 0.0 2e+01))
  (Variables|Default|SetSpawnTime (* (Variables|Default|GetSpawnTime) 0.95)))

(fn ConstructionScript)

(fn RandomTransform
  (bind _returnvalue (Math|Random|RandomFloatinRange 0.0 3.6e+02))
  (bind _spawnradius (Variables|Default|GetSpawnRadius))
  (return (Math|Transform|MakeTransform (+ (Math|Vector|MakeVector (* (Math|Trig|Cos(Degrees) _returnvalue) _spawnradius) (* (Math|Trig|Sin(Degrees) _returnvalue) _spawnradius) 0.0) (Transformation|GetActorLocation (Game|Player|GetPlayerPawn 0))))))