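; U_Defender is a Golem unit Blueprint for a defender that is bound to the player pawn.
; BeginPlay sets walk speed, attaches the unit to player pawn 0 keeping world transform, and stores its offset from that pawn as Anchor.
; Tick defers to the parent class.
; Attack checks health and cooldown but performs no action, as the cooldown timer reset is left disconnected.
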(event EventBeginPlay
  (Variables|/Script/Engine.CharacterMovementComponent|SetMaxWalkSpeed (Variables|Character|GetCharacterMovement) (Variables|Default|GetMovementSpeed))
  (Transformation|AttachActorToActor (Game|Player|GetPlayerPawn 0) "None" "KeepWorld" "KeepWorld" "KeepWorld" true)
  (Variables|Default|SetAnchor (- (Transformation|GetActorLocation self) (Transformation|GetActorLocation (Game|Player|GetPlayerPawn 0)))))

(event Collision|EventActorBeginOverlap
  (params (OtherActor :type Actor%20Object%20Reference)))

(event EventTick
  (params (DeltaSeconds :type Float%20%28single-precision%29))
  (|CallParentFunction DeltaSeconds))

(event EventAttack
  (if (> (Variables|Default|GetHealth) 0.0)
    (if (> (Variables|Default|GetTimeSinceLastAttack) (Variables|Default|GetAttackCoolDown))
      _)))

(fn ConstructionScript
  (|CallParentFunction))