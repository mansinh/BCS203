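; Behavior tree task that points a Unit's AI controller at its target and records the target's location.
; The focal point is set to the TargetActor's location when valid, otherwise to the Location blackboard value.
; Both branches then write the TargetActor's location to that key, even if invalid, and finish successfully.
; A failed Unit cast stops execution without finishing the task.
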(event EventReceiveExecuteAI
  (params (OwnerController :type AI%20Controller%20Object%20Reference) (ControlledPawn :type Pawn%20Object%20Reference))
  (bind _asunit (Utilities|Casting|CastToUnit ControlledPawn))
  (Utilities|IsValid (Variables|/Game/Golem/Blueprints/Units/Unit.Unit_C|GetTargetActor _asunit)
    (:Is%20Valid
      (AI|SetFocalPoint OwnerController (Transformation|GetActorLocation (Variables|/Game/Golem/Blueprints/Units/Unit.Unit_C|GetTargetActor _asunit))))
    (:Is%20Not%20Valid
      (AI|SetFocalPoint OwnerController (Class|BTFunctionLibrary|GetBlackboardValueasVector (Variables|Default|GetLocation)))))
  (AI|BehaviorTree|SetBlackboardValueasVector (Variables|Default|GetLocation) (Transformation|GetActorLocation (Variables|/Game/Golem/Blueprints/Units/Unit.Unit_C|GetTargetActor _asunit)))
  (AI|BehaviorTree|FinishExecute true))