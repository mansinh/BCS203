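; U_Mage is a ranged mage unit that attaches to the player pawn on BeginPlay and records its offset as an anchor.
; ShootTarget aims the fire point just above the target's origin, checks line of sight, then activates a particle effect and spawns a projectile.
; The Attack event checks health and cooldown but performs no action.
; The fire sound and cooldown reset are disconnected, and nothing here calls ShootTarget.
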(event EventBeginPlay
  (Variables|/Script/Engine.CharacterMovementComponent|SetMaxWalkSpeed (Variables|Character|GetCharacterMovement) (Variables|Default|GetMovementSpeed))
  (Transformation|AttachActorToActor (Game|Player|GetPlayerPawn 0) "None" "KeepWorld" "KeepWorld" "KeepWorld" true)
  (Variables|Default|SetAnchor (- (Transformation|GetActorLocation self) (Transformation|GetActorLocation (Game|Player|GetPlayerPawn 0)))))

(event Collision|EventActorBeginOverlap
  (params (OtherActor :type Actor%20Object%20Reference)))

(event EventTick
  (params (DeltaSeconds :type Float%20%28single-precision%29))
  (|CallParentFunction DeltaSeconds))

(event EventAttack
  (if (> (Variables|Default|GetHealth) 0.0)
    (if (> (Variables|Default|GetTimeSinceLastAttack) (Variables|Default|GetAttackCoolDown))
      _)))

(fn ConstructionScript
  (|CallParentFunction))

(fn ShootTarget
  (bind _targetactor (Variables|Default|GetTargetActor))
  (bind _shootfromposition (Variables|Default|GetShootFromPosition))
  (bind _returnvalue (Transformation|GetActorLocation _targetactor))
  (bind _returnvalue_2 (Transformation|GetWorldLocation _shootfromposition))
  (bind _returnvalue_3 (+ _returnvalue (Math|Vector|MakeVector 0.0 0.0 1e+01)))
  (Utilities|IsValid self
    (:Is%20Valid
      (Utilities|IsValid _targetactor
        (:Is%20Valid
          (Transformation|SetWorldRotation _shootfromposition (Math|Rotator|FindLookatRotation _returnvalue_2 _returnvalue_3) false false)
          (bind _result (CallFunction|HasLineOfSight _returnvalue_2 _returnvalue_3 (Utilities|Array|MakeArray self _targetactor)))
          (if _result
            (Components|Activation|Activate (Variables|Default|GetParticleSystem_0) true)
            (Game|SpawnActorfromClass "/Game/Golem/Blueprints/Units/UnitProjectile.UnitProjectile_C" (Transformation|GetWorldTransform (Variables|Default|GetShootFromPosition)) "AlwaysSpawn" 0 (Variables|Default|GetProjectileSpeed) 0)))))))