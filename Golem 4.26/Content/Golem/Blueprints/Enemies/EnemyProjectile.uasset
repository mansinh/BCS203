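; Enemy projectile that deals damage on hit to player units and other Units, with zero knockback.
; The construction script copies Speed into the projectile movement's initial speed.
; The Hit event casts to PlayerUnit first, then Unit, sending the former an attack message and calling Attacked on the latter.
; A unit hit activates the Hit effect, hides the mesh and disables collision, then briefly delays before destroying the actor.
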(event Collision|EventHit
  (params (MyComp :type Primitive%20Component%20Object%20Reference) (Other :type Actor%20Object%20Reference) (OtherComp :type Primitive%20Component%20Object%20Reference) (bSelfMoved :type Boolean) (HitLocation :type Vector :default "0, 0, 0") (HitNormal :type Vector :default "0, 0, 0") (NormalImpulse :type Vector :default "0, 0, 0") (Hit :type Hit%20Result%20Structure%20%28by%20ref%29))
  (bind _attackdamage (Variables|Default|GetAttackDamage))
  (Utilities|IsValid Other
    (:Is%20Valid
      (Utilities|IsValid OtherComp
        (:Is%20Valid
          (bind _asplayer_unit (Utilities|Casting|CastToPlayerUnit Other)
            (:then
              (Class|GolemInterface|Attacked(Message) _asplayer_unit _attackdamage "0, 0, 0")
              (Components|Activation|Activate (Variables|Default|GetHit) true :!label _label)
              (Rendering|SetVisibility (Variables|Default|GetProjectileMesh) false false)
              (Collision|SetActorEnableCollision false)
              (Utilities|FlowControl|Delay 0.2))
            (:CastFailed
              (bind _asunit (Utilities|Casting|CastToUnit Other)
                (:then
                  (Default|Attacked _asunit _attackdamage "0, 0, 0")
                  (goto _label))
                (:CastFailed
                  _))))
          (Actor|DestroyActor))
        (:Is%20Not%20Valid)))
    (:Is%20Not%20Valid)))

(fn ConstructionScript
  (Variables|/Script/Engine.ProjectileMovementComponent|SetInitialSpeed (Variables|Default|GetProjectileMovement) (Variables|Default|GetSpeed)))